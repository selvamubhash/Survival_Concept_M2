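; BP_Projectile_02 is an inventory-system projectile that deals damage and leaves bullet holes on impact.
; On its first hit with authority, it applies damage from CalculateDamage to the hit actor, skipping its own instigator, then destroys itself.
; A separate sequence branch attaches a bullet-hole decal with a randomized lifespan to WorldStatic surfaces, oriented along the hit normal, without an authority check.
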(event Collision|EventHit
  (params (MyComp :type Primitive%20Component%20Object%20Reference) (Other :type Actor%20Object%20Reference) (OtherComp :type Primitive%20Component%20Object%20Reference) (bSelfMoved :type Boolean) (HitLocation :type Vector :default "0, 0, 0") (HitNormal :type Vector :default "0, 0, 0") (NormalImpulse :type Vector :default "0, 0, 0") (Hit :type Hit%20Result%20Structure%20%28by%20ref%29))
  ;[1 1 1] On Projectile Hit
  (Utilities|FlowControl|Sequence
    (:then_0
      (Networking|SwitchHasAuthority
        (:Authority
          (Utilities|FlowControl|DoOnce false
            (:Completed
              (if (!= (Game|GetInstigator) Other)
                (Game|Damage|ApplyDamage Other (CallFunction|CalculateDamage Hit) (Pawn|GetController (Game|GetInstigator)) 0 "/Script/Engine.DamageType")
                (Actor|DestroyActor)
                (else
                  (Actor|DestroyActor))))))))
    (:then_1
      (if (Utilities|Enum|Equal(Enum) (Collision|GetCollisionObjectType OtherComp) "ECC_WorldStatic")
        (Class|GameplayStatics|SpawnDecalAttached "/Game/AdvancedInventory/otherStuff/Materials/Other/M_BulletHoleDecal.M_BulletHoleDecal" "18.000000,12.000000,12.000000" OtherComp "None" HitLocation (Math|Conversions|RotationFromXVector HitNormal) "KeepWorldPosition" (Math|Conversions|ToFloat(Integer) (Math|Random|RandomIntegerinRange 7 12)))))))

(fn ConstructionScript
  (|CallParentFunction))