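; Base projectile Blueprint for the inventory system's weapons, holding damage and a headshot multiplier supplied through SetUp.
; BeginPlay enables query-only collision on the Sphere after a very short delay, so bullets avoid sticking in their own shooter at higher ping.
; CalculateDamage applies the multiplier when the hit bone is "head".
; The OnRep for the bullet hole flag is empty here.
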(event EventBeginPlay
  ;[1 1 1] initially without collsion to prevent bullet to stuck in own player if running forward, with higher pings. To reduce the problem, you can also reduce the Sphere size or  move the
  ; muzzle socket in the weapon further away from the character
  (Utilities|FlowControl|Delay 0.005)
  (Collision|SetCollisionEnabled (Variables|Default|GetSphere) "QueryOnly"))

(fn ConstructionScript)

(fn OnRepBSpawnBulletHole)

(fn CalculateDamage
  (params (Hit :type Hit%20Result%20Structure%20%28by%20ref%29))
  (return (select (Utilities|Name|Equal(Name) (.HitBoneName (Collision|BreakHitResult Hit)) "head") (* (Variables|Default|GetDamage) (Variables|Default|GetHeadShotMultiplier)) (Variables|Default|GetDamage))))

(fn SetUp
  (params (Damage :type Float%20%28double-precision%29) (HeadShotMultiplier :type Float%20%28double-precision%29))
  (Variables|Default|SetDamage Damage)
  (Variables|Default|SetHeadShotMultiplier HeadShotMultiplier))