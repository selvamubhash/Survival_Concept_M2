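; Server-authoritative item spawner that periodically drops a configured data table item as a BP_DropItemActor with random yaw at its spawn location.
; BeginPlay validates the row, then UpdateInterval sets the actor tick interval so Tick serves as the spawn timer.
; Before each spawn, a sphere trace around the density check point caps nearby matching items, using stack amount for stackables and actor count for non-stackables.
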(event Custom|SpawnItemOnServer
  ;[1 1 1] Spawn item on server
  (if (Variables|Default|GetbSpawningEnabled)
    (bind _belowmaxdensity (CallFunction|DensityReachedCheck))
    (if _belowmaxdensity
      (if (Variables|Default|GetbSetUpValid)
        (Game|SpawnActorfromClass "/Game/AdvancedInventory/Blueprints/General/BP_DropItemActor.BP_DropItemActor_C" (Math|Transform|MakeTransform (Transformation|GetWorldLocation (Variables|Default|GetSpawnLocation)) (Math|Rotator|MakeRotator 0.0 0.0 (Math|Conversions|ToFloat(Integer) (Math|Random|RandomIntegerinRange 0 360)))) "Undefined" "OverrideRootScale" 0 (Utilities|Struct|MakeS_SpawnItemSettings true (Variables|Default|GetItemToSpawn)) (Variables|Default|GetAmountToSpawn) 0.0 false 0)))))

(event EventTick
  (params (DeltaSeconds :type Float%20%28single-precision%29))
  ;[1 1 1] Event Tick is set to Spawn Interval (so it is not firing each frame)
  (Networking|SwitchHasAuthority
    (:Authority
      (CallFunction|SpawnItemonServer))))

(event EventBeginPlay
  (bind _itemtospawn (Variables|Default|GetItemToSpawn))
  (bind (_datatable _rowname) (Utilities|Struct|BreakDataTableRowHandle _itemtospawn))
  ;[1 1 1] Set up
  (Networking|SwitchHasAuthority
    (:Authority
      (bind _returnvalue (Utilities|GetDataTableRow _datatable _rowname)
        (:then
          (bind _output_get (Variables|Default|SetItemDataToSpawn _returnvalue))
          (Utilities|Struct|SetmembersinS_ItemData _output_get (Variables|Default|GetAmountToSpawn))
          (Variables|Default|SetbSetUpValid true)
          (if (Variables|Default|GetbSpawningEnabled)
            (CallFunction|UpdateInterval (Variables|Default|GetSpawnInterval))))))))

(fn ConstructionScript)

(fn UpdateInterval
  (params (TickInterval :type Float%20%28double-precision%29))
  (bind _output_get (Variables|Default|SetSpawnInterval TickInterval))
  (Actor|Tick|SetActorTickInterval _output_get)
  (Actor|Tick|SetActorTickEnabled true))

(fn DensityReachedCheck
  (bind _densitychecklocation (Variables|Default|GetDensityCheckLocation))
  (bind _returnvalue (Transformation|GetWorldLocation _densitychecklocation))
  ;[1 1 1] Trace items next to spawner and check if the amount is smaller than the maximum threshold (MaximumAmountDensity)
  (if (> (Variables|Default|GetMaximumAmountDensity) 0)
    (bind (_outhits _returnvalue_2) (Collision|MultiSphereTraceForObjects _returnvalue (- _returnvalue "0, 0,22.000000") 1.3e+02 (Utilities|Array|MakeArray "ObjectTypeQuery9") false 0 "None" true "(R=1.000000,G=0.000000,B=0.000000,A=1.000000)" "(R=0.000000,G=1.000000,B=0.000000,A=1.000000)" 0.5))
    (if _returnvalue_2
      (for _array_element _outhits
        (bind _asbp_drop_item_actor (Utilities|Casting|CastToBP_DropItemActor (.HitActor (Collision|BreakHitResult _array_element))))
        (if (Utilities|Name|Equal(Name) (Utilities|Struct|BreakDataTableRowHandle (Variables|Default|GetItemToSpawn)) (.ID (Utilities|Struct|BreakS_ItemData (Variables|/Game/AdvancedInventory/Blueprints/General/BP_DropItemActor.BP_DropItemActor_C|GetItemDataNew _asbp_drop_item_actor))))
          (if (Utilities|Struct|BreakS_AdditionalGeneralData (.AdditionalGeneralData (Utilities|Struct|BreakS_ItemData (Variables|/Game/AdvancedInventory/Blueprints/General/BP_DropItemActor.BP_DropItemActor_C|GetItemDataNew _asbp_drop_item_actor))))
            (if (>= (.Amount (Utilities|Struct|BreakS_ItemData (Variables|/Game/AdvancedInventory/Blueprints/General/BP_DropItemActor.BP_DropItemActor_C|GetItemDataNew _asbp_drop_item_actor))) (Variables|Default|GetMaximumAmountDensity))
              (return false))
            (else
              (Math|Integer|IncrementInt (LocalVariables|GetNonStackableSum))))))
      (return (<= (LocalVariables|GetNonStackableSum) (Variables|Default|GetMaximumAmountDensity)))
      (else
        (return true)))
    (else
      (return true))))