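; Torch item child actor with a particle effect and point light, activating the particles shortly after BeginPlay.
; When its parent component is tagged "inspector", it stops the flicker timeline and destroys the light.
; A FlickeringLight timeline holds logic to scale light intensity from a default value.
; An unconnected UE4 workaround would destroy the torch along with its parent actor.
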(event Custom|OnDestroyed_Event_0
  (params (DestroyedActor :type Actor%20Object%20Reference))
  ;[1 1 1] only necessary in ue4 because of an engine bug where child actor won't get destroyed if their parent actor gets destryoed
  (Actor|DestroyActor))

(event EventBeginPlay
  (CallFunction|DestroyLigthifUsedinInspector)
  (Utilities|FlowControl|Delay 0.1)
  (Components|Activation|Activate (Variables|Default|GetParticleSystem) false))

(fn ConstructionScript)

(fn DestroyLigthifUsedinInspector
  (if (Utilities|Array|ContainsItem (Variables|/Script/Engine.ActorComponent|GetComponentTags (Class|Actor|GetParentComponent)) "inspector")
    (Audio|Components|Audio|Stop (Variables|Default|GetFlickeringLight))
    (Components|DestroyComponent (Variables|Default|GetPointLight))))