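; Server-side cooking component for BP_0_Chest_Master chests such as campfires, which turns items in cooking slots into cooked results while burning fuel.
; The chest's flat slot array is split into cooking, fuel and content sections, with items stored as strings.
; A looping timer advances per-slot progress, consumes fuel and stacks finished items into content slots.
; Progress and slot changes are pushed only to players currently interacting with that chest.
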(event Custom|CheckCooking
  (params (ResetSecondsCooked :type Boolean) (ResetSlot :type Integer))
  ;[1 1 1] Updates on server
  (General|ChecktoStartCooking ResetSecondsCooked))

(event Custom|UpdateCookingProgressOnServer
  (params (Percent :type Array%20of%20Integers) (TurnOffCampfire :type Boolean))
  ;[1 1 1] Updates on server
  (Updating|UpdateCookingProgress Percent TurnOffCampfire))

(event Custom|RemoveAndAddCampfireItem
  (params (RemoveAtCookingSlot :type Array%20of%20Integers))
  ;[1 1 1] Updates on server
  (Updating|RemoveandAdd RemoveAtCookingSlot))

(event EventBeginPlay
  ;[1 1 1] Event BeginPlay
  (SetUp|SetUp))

(fn GetFirstSlotwithSameIDorEmptySlotandUpdate
  (params (ID :type Name) (UpdateItemDataInSameStep :type Boolean) (AmountToCook :type Integer))
  ;[1 1 1] Set up local variables
  (LocalVariables|SetID_Local ID)
  (LocalVariables|SetUpdateDataInSameStep UpdateItemDataInSameStep)
  (LocalVariables|SetAmoutToCook_Local AmountToCook)
  ;[1 1 1] Get default item data of item that should be added
  (bind (_out_row _found) (CallFunction|GetItemDatabyID (LocalVariables|GetID_Local)))
  (if _found
    (LocalVariables|SetItemToAdd _out_row)
    ;[1 1 1] Check if item to add is stackable
    (if (Utilities|Struct|BreakS_AdditionalGeneralData (Utilities|Struct|BreakS_ItemData (LocalVariables|GetItemToAdd)))
      ;[1 1 1] Search for visible item that is not fully stacked
      ;;[1 1 1] Loop: only visible items in content section
      (for (_array_element _array_index) (Variables|/Game/AdvancedInventory/Blueprints/Chests/BP_0_Chest_Master.BP_0_Chest_Master_C|GetVisibility_AllSlots (Variables|General|GetParentChestRef))
        (LocalVariables|SetL_Index _array_index)
        (if (>= (LocalVariables|GetL_Index) (Other|GetFirstContentSlotIndex))
          (if _array_element
            (bind _output_get (LocalVariables|SetCompareLoopItemData (Other|GetChestItemDatabyIndex (LocalVariables|GetL_Index))))
            (if (Utilities|Name|Equal(Name) (LocalVariables|GetID_Local) (Utilities|Struct|BreakS_ItemData _output_get))
              (if (<= (+ (.Amount (Utilities|Struct|BreakS_ItemData (LocalVariables|GetCompareLoopItemData))) (LocalVariables|GetAmoutToCook_Local)) (Utilities|Struct|BreakS_AdditionalGeneralData (.AdditionalGeneralData (Utilities|Struct|BreakS_ItemData (LocalVariables|GetCompareLoopItemData)))))
                (if (LocalVariables|GetUpdateDataInSameStep)
                  ;;[1 1 1] Add item to found slot
                  (Utilities|Struct|SetmembersinS_AdditionalGeneralData (Utilities|Struct|BreakS_ItemData (LocalVariables|GetItemToAdd)) (Utilities|Struct|BreakS_AdditionalGeneralData (Utilities|Struct|BreakS_ItemData (LocalVariables|GetCompareLoopItemData))))
                  (bind _structout (Utilities|Struct|SetmembersinS_ItemData (LocalVariables|GetItemToAdd) (+ (Utilities|Struct|BreakS_ItemData (LocalVariables|GetCompareLoopItemData)) (LocalVariables|GetAmoutToCook_Local))))
                  (Updating|UpdateChestItemDatabyIndex (LocalVariables|GetL_Index) _structout)
                  (Utilities|Array|Add (Variables|CookingResult|GetSlotsToAdd) (LocalVariables|GetL_Index))
                  (Utilities|Array|Add (Variables|CookingResult|GetItemsToAdd) (CallFunction|ItemDatatoString (LocalVariables|GetItemToAdd)))
                  (return true (LocalVariables|GetL_Index))
                  (else
                    ;;[1 1 1] just return found slot
                    (return true (LocalVariables|GetL_Index))))
                (elif (< (.Amount (Utilities|Struct|BreakS_ItemData (LocalVariables|GetCompareLoopItemData))) (Utilities|Struct|BreakS_AdditionalGeneralData (.AdditionalGeneralData (Utilities|Struct|BreakS_ItemData (LocalVariables|GetCompareLoopItemData))))) ; check if stack is not full
                  (LocalVariables|SetAmountToCookLeft_Local (- (+ (.Amount (Utilities|Struct|BreakS_ItemData (LocalVariables|GetCompareLoopItemData))) (LocalVariables|GetAmoutToCook_Local)) (Utilities|Struct|BreakS_AdditionalGeneralData (.AdditionalGeneralData (Utilities|Struct|BreakS_ItemData (LocalVariables|GetCompareLoopItemData))))))
                  (if (LocalVariables|GetUpdateDataInSameStep)
                    ;;[1 1 1] Fill up item amount to maximum stack size
                    (Utilities|Struct|SetmembersinS_AdditionalGeneralData (Utilities|Struct|BreakS_ItemData (LocalVariables|GetItemToAdd)) (.UniqueReplicationID (Utilities|Struct|BreakS_AdditionalGeneralData (Utilities|Struct|BreakS_ItemData (LocalVariables|GetCompareLoopItemData)))))
                    (bind _structout_2 (Utilities|Struct|SetmembersinS_ItemData (LocalVariables|GetItemToAdd) (Utilities|Struct|BreakS_AdditionalGeneralData (Utilities|Struct|BreakS_ItemData (LocalVariables|GetCompareLoopItemData)))))
                    (Updating|UpdateChestItemDatabyIndex (LocalVariables|GetL_Index) _structout_2)
                    (Utilities|Array|Add (Variables|CookingResult|GetSlotsToAdd) (LocalVariables|GetL_Index))
                    (Utilities|Array|Add (Variables|CookingResult|GetItemsToAdd) (CallFunction|ItemDatatoString (LocalVariables|GetItemToAdd)))
                    (LocalVariables|SetAmoutToCook_Local (LocalVariables|GetAmountToCookLeft_Local))
                    (LocalVariables|SetAmountToCookLeft_Local 0)
                    (LocalVariables|SetneedAdditionalUpdate true)))))))))
    ;[1 1 1] Search for empty slot
    ;;[1 1 1] Loop: only empty slots in content section
    (for (_array_element_2 _array_index_2) (Variables|/Game/AdvancedInventory/Blueprints/Chests/BP_0_Chest_Master.BP_0_Chest_Master_C|GetVisibility_AllSlots (Variables|General|GetParentChestRef))
      (LocalVariables|SetL_Index _array_index_2)
      (if (>= (LocalVariables|GetL_Index) (Other|GetFirstContentSlotIndex))
        (if (not _array_element_2)
          (if (LocalVariables|GetUpdateDataInSameStep)
            ;;[1 1 1] Add item to empty slot
            (Utilities|Array|SetArrayElem (Variables|/Game/AdvancedInventory/Blueprints/Chests/BP_0_Chest_Master.BP_0_Chest_Master_C|GetVisibility_AllSlots (Variables|General|GetParentChestRef)) (LocalVariables|GetL_Index) true)
            (Utilities|Struct|SetmembersinS_AdditionalGeneralData (Utilities|Struct|BreakS_ItemData (LocalVariables|GetItemToAdd)) (Other|GenerateUniqueID (LocalVariables|GetID_Local)))
            (bind _structout_3 (Utilities|Struct|SetmembersinS_ItemData (LocalVariables|GetItemToAdd) (LocalVariables|GetAmoutToCook_Local)))
            (Updating|UpdateChestItemDatabyIndex (LocalVariables|GetL_Index) _structout_3)
            (Utilities|Array|Add (Variables|CookingResult|GetSlotsToAdd) (LocalVariables|GetL_Index))
            (Utilities|Array|Add (Variables|CookingResult|GetItemsToAdd) (CallFunction|ItemDatatoString (LocalVariables|GetItemToAdd)))
            (return true (LocalVariables|GetL_Index))
            (else
              ;;[1 1 1] just return found slot
              (return true (LocalVariables|GetL_Index)))))))
    (return (LocalVariables|GetneedAdditionalUpdate) 0)))

(fn GetPercentOfAllCookingSlots
  ;[1 1 1] Update percent progress array
  (for (_array_element _array_index) (Variables|CookingSlots|GetSecondsCookedArray)
    (if (> (Utilities|Array|Get(acopy) (Variables|CookingSlots|GetSecondsToCookArray) _array_index) 0.0)
      (Utilities|Array|Add (LocalVariables|GetLocalPercentArray) (Math|Integer|Clamp(Integer) (Math|Float|Truncate (* (/ _array_element (Utilities|Array|Get(acopy) (Variables|CookingSlots|GetSecondsToCookArray) _array_index)) 1e+02)) 0 100))
      (else
        (Utilities|Array|Add (LocalVariables|GetLocalPercentArray) 0))))
  (return (LocalVariables|GetLocalPercentArray)))

(fn SetDecreaseCookingArrayFalse
  ;[1 1 1] Reset array
  (for _index (range 0 (- (Utilities|Array|Length (Variables|CookingSlots|GetDecreaseCookingSlotArray)) 1))
    (Utilities|Array|SetArrayElem (Variables|CookingSlots|GetDecreaseCookingSlotArray) _index false)))

(fn AllCookingSlotstoZero
  ;[1 1 1] reset percent array
  (for _index (range 0 (- (Utilities|Array|Length (Variables|CookingSlots|GetSecondsToCookArray)) 1))
    (Utilities|Array|Add (LocalVariables|GetlocalPercent) 0))
  (return (LocalVariables|GetlocalPercent)))

(fn HasPlaceinContentSection
  (for _index (range 0 (- (Utilities|Struct|BreakS_ChestCookingModule (Variables|/Game/AdvancedInventory/Blueprints/Chests/BP_0_Chest_Master.BP_0_Chest_Master_C|GetCookingModule (Variables|General|GetParentChestRef))) 1))
    (if (Utilities|Array|Get(acopy) (Variables|/Game/AdvancedInventory/Blueprints/Chests/BP_0_Chest_Master.BP_0_Chest_Master_C|GetVisibility_AllSlots (Variables|General|GetParentChestRef)) _index)
      (bind _found_ (Updating|GetFirstSlotwithSameIDorEmptySlotandUpdate (Utilities|Struct|BreakS_ItemData (CallFunction|StringtoItemData (Utilities|Array|Get(acopy) (Variables|/Game/AdvancedInventory/Blueprints/Chests/BP_0_Chest_Master.BP_0_Chest_Master_C|GetItemString_AllSlots (Variables|General|GetParentChestRef)) _index))) false))
      (if _found_
        (return true))))
  (return false))

(fn FindFuelItemandUpdate
  ;[1 1 1] Loop: Visible items in fuel section
  (for (_array_element _array_index) (Variables|/Game/AdvancedInventory/Blueprints/Chests/BP_0_Chest_Master.BP_0_Chest_Master_C|GetVisibility_AllSlots (Variables|General|GetParentChestRef))
    (bind _output_get (LocalVariables|SetIndex _array_index))
    (if (Other|CheckifFuelIndex _output_get)
      (if _array_element
        ;[1 1 1] only continue if item has actually fuel
        (LocalVariables|SetLocalItemData (Other|GetChestItemDatabyIndex (LocalVariables|GetIndex)))
        (if (> (.FuelAmount (Utilities|Struct|BreakS_Cooking (Utilities|Struct|BreakS_ItemData (LocalVariables|GetLocalItemData)))) 0.0)
          ;[1 1 1] Decrease fuel item amount by 1 and clear it if it becomes 0
          (if (<= (- (Utilities|Struct|BreakS_ItemData (LocalVariables|GetLocalItemData)) 1) 0)
            (Utilities|Array|SetArrayElem (Variables|/Game/AdvancedInventory/Blueprints/Chests/BP_0_Chest_Master.BP_0_Chest_Master_C|GetVisibility_AllSlots (Variables|General|GetParentChestRef)) (LocalVariables|GetIndex) false)
            (else
              (bind _structout (Utilities|Struct|SetmembersinS_ItemData (LocalVariables|GetLocalItemData) (- (Utilities|Struct|BreakS_ItemData (LocalVariables|GetLocalItemData)) 1)))
              (Updating|UpdateChestItemDatabyIndex (LocalVariables|GetIndex) _structout)))
          (return true (.FuelAmount (Utilities|Struct|BreakS_Cooking (Utilities|Struct|BreakS_ItemData (LocalVariables|GetLocalItemData)))) (LocalVariables|GetIndex))
          (else
            (return false 0.0 0))))))
  (return false 0.0 0))

(fn RemoveandAdd
  (params (RemoveAtCookingSlot :type Array%20of%20Integers))
  ;[1 1 1] Reset arrays
  (Other|SetDecreaseCookingArrayFalse)
  (Utilities|Array|Clear (Variables|CookingResult|GetSlotsToAdd))
  (Utilities|Array|Clear (Variables|CookingResult|GetItemsToAdd))
  ;[1 1 1] Add resulting items to content section
  (for _array_element RemoveAtCookingSlot
    (bind _output_get (LocalVariables|SetIndex _array_element))
    (bind _output_get_2 (LocalVariables|SetItemData (Other|GetChestItemDatabyIndex _output_get)))
    (bind _found_ (Updating|GetFirstSlotwithSameIDorEmptySlotandUpdate (Utilities|Struct|BreakDataTableRowHandle (.ItemToCook (Utilities|Struct|BreakS_Cooking (Utilities|Struct|BreakS_ItemData _output_get_2)))) true (.AmountToCook (Utilities|Struct|BreakS_Cooking (Utilities|Struct|BreakS_ItemData _output_get_2)))))
    (if _found_
      (Utilities|Array|SetArrayElem (Variables|CookingSlots|GetSecondsCookedArray) (LocalVariables|GetIndex) 0.0)
      (Utilities|Array|SetArrayElem (Variables|CookingSlots|GetDecreaseCookingSlotArray) (LocalVariables|GetIndex) true)
      ;[1 1 1] Decrease Cooking slots item amount
      (if (<= (- (Utilities|Struct|BreakS_ItemData (LocalVariables|GetItemData)) 1) 0)
        (Utilities|Array|SetArrayElem (Variables|/Game/AdvancedInventory/Blueprints/Chests/BP_0_Chest_Master.BP_0_Chest_Master_C|GetVisibility_AllSlots (Variables|General|GetParentChestRef)) (LocalVariables|GetIndex) false)
        (else
          (bind _structout (Utilities|Struct|SetmembersinS_ItemData (LocalVariables|GetItemData) (- (Utilities|Struct|BreakS_ItemData (LocalVariables|GetItemData)) 1)))
          (Updating|UpdateChestItemDatabyIndex (LocalVariables|GetIndex) _structout)))))
  ;[1 1 1] Update cooking UI and eventually sto cooking
  (Updating|UpdateCookingUIforAllPlayers (Utilities|Struct|MakeS_ChestCookingUpdateData (GetCookingData|GetPercentOfAllCookingSlots) (Variables|CookingSlots|GetDecreaseCookingSlotArray) (Variables|CookingResult|GetSlotsToAdd) (Variables|CookingResult|GetItemsToAdd)))
  (if (GetCookingData|HasPlaceinContentSection)
    (if (not (GetCookingData|HasCookingItem))
      (General|StopCooking))
    (else
      (General|StopCooking))))

(fn UpdateSecondstoCookArray
  ;[1 1 1] Update seconds to cook array: this is the duration that is needed to cook, NOT the cooking progress
  (for _index (range 0 (- (Utilities|Array|Length (Variables|CookingSlots|GetSecondsToCookArray)) 1))
    (if (Utilities|Array|Get(acopy) (Variables|/Game/AdvancedInventory/Blueprints/Chests/BP_0_Chest_Master.BP_0_Chest_Master_C|GetVisibility_AllSlots (Variables|General|GetParentChestRef)) _index)
      (Utilities|Array|SetArrayElem (Variables|CookingSlots|GetSecondsToCookArray) _index (.DurationToCookInSeconds (Utilities|Struct|BreakS_Cooking (Utilities|Struct|BreakS_ItemData (CallFunction|StringtoItemData (Utilities|Array|Get(acopy) (Variables|/Game/AdvancedInventory/Blueprints/Chests/BP_0_Chest_Master.BP_0_Chest_Master_C|GetItemString_AllSlots (Variables|General|GetParentChestRef)) _index))))))
      (else
        (Utilities|Array|SetArrayElem (Variables|CookingSlots|GetSecondsToCookArray) _index 0.0)))))

(fn HasCookingItem
  ;[1 1 1] check if any item is placed in any cooking slot
  (for _index (range 0 (- (Utilities|Struct|BreakS_ChestCookingModule (Variables|/Game/AdvancedInventory/Blueprints/Chests/BP_0_Chest_Master.BP_0_Chest_Master_C|GetCookingModule (Variables|General|GetParentChestRef))) 1))
    (if (Utilities|Array|Get(acopy) (Variables|/Game/AdvancedInventory/Blueprints/Chests/BP_0_Chest_Master.BP_0_Chest_Master_C|GetVisibility_AllSlots (Variables|General|GetParentChestRef)) _index)
      (return true)))
  (return false))

(fn ChecktoStartCooking
  (params (ResetSecondsCokked :type Boolean))
  ;[1 1 1] Start/Stop cooking if there is a cooking item and fuel
  (if (GetCookingData|HasCookingItem)
    (if ResetSecondsCokked
      _
      (else
        _))
    (Updating|UpdateSecondstoCookArray)
    (if (not (Variables|General|GetbCooking))
      (if (> (Variables|General|GetFuel) 0.0)
        (Updating|UpdateCookingUIforAllPlayers (Utilities|Struct|MakeS_ChestCookingUpdateData true (stale _itemindex)) :!label _label)
        (Variables|General|SetbCooking true)
        (bind _returnvalue (Utilities|Time|SetTimerbyFunctionName 0 "StartCooking" (Variables|General|GetCookInterval) true))
        (Variables|General|SetCookTimer _returnvalue)
        (Default|CallOnCookingTurnedon (Variables|General|GetParentChestRef) true)
        (else
          (bind (_found _fuelamount _itemindex) (Updating|FindFuelItemandUpdate))
          (if _found
            (Variables|General|SetFuel _fuelamount)
            (goto _label)))))
    (else
      (Default|CallOnCookingTurnedon (Variables|General|GetParentChestRef) false)
      (Variables|General|SetbCooking false))))

(fn StartCooking
  ;[1 1 1] Update cooking progress
  (for (_array_element _array_index) (Variables|CookingSlots|GetSecondsCookedArray)
    (LocalVariables|SetIndex _array_index)
    (if (Utilities|Array|Get(acopy) (Variables|/Game/AdvancedInventory/Blueprints/Chests/BP_0_Chest_Master.BP_0_Chest_Master_C|GetVisibility_AllSlots (Variables|General|GetParentChestRef)) (LocalVariables|GetIndex))
      (Utilities|Array|SetArrayElem (Variables|CookingSlots|GetSecondsCookedArray) (LocalVariables|GetIndex) (+ _array_element (Variables|General|GetCookInterval)))
      (if (>= (Utilities|Array|Get(acopy) (Variables|CookingSlots|GetSecondsCookedArray) (LocalVariables|GetIndex)) (Utilities|Array|Get(acopy) (Variables|CookingSlots|GetSecondsToCookArray) (LocalVariables|GetIndex)))
        (Utilities|Array|Add (LocalVariables|GetLocalCookingItemIndexesToDecrease) (LocalVariables|GetIndex)))
      (else
        (Utilities|Array|SetArrayElem (Variables|CookingSlots|GetSecondsCookedArray) (LocalVariables|GetIndex) 0.0))))
  ;[1 1 1] Check if any progress is complete
  (if (> (Utilities|Array|Length (LocalVariables|GetLocalCookingItemIndexesToDecrease)) 0)
    (CallFunction|RemoveandAddCampfireItem (LocalVariables|GetLocalCookingItemIndexesToDecrease)))
  (CallFunction|UpdateCookingProgressonServer (GetCookingData|GetPercentOfAllCookingSlots) (not (GetCookingData|HasCookingItem))))

(fn SetUp
  ;[1 1 1] add reference variables
  (Utilities|IsValid (Game|GetGameMode) ; Set up only on server
    (:Is%20Valid
      (Variables|Default|SetGameModeComponentRef (Actor|GetComponentbyClass (Game|GetGameMode) "/Game/AdvancedInventory/Blueprints/Components/AC_InventoryGameMode_Component.AC_InventoryGameMode_Component_C"))
      (bind _asbp_0_chest_master (Utilities|Casting|CastToBP_0_Chest_Master (Components|GetOwner)))
      (Variables|General|SetParentChestRef _asbp_0_chest_master)
      ;[1 1 1] Set up empty cooking slot arrays
      (for _index (range 0 (- (Utilities|Struct|BreakS_ChestCookingModule (Variables|/Game/AdvancedInventory/Blueprints/Chests/BP_0_Chest_Master.BP_0_Chest_Master_C|GetCookingModule (Variables|General|GetParentChestRef))) 1))
        (Utilities|Array|Add (Variables|CookingSlots|GetSecondsCookedArray) 0.0)
        (Utilities|Array|Add (Variables|CookingSlots|GetSecondsToCookArray) 0.0)
        (Utilities|Array|Add (Variables|CookingSlots|GetDecreaseCookingSlotArray) false)))))

(fn CheckifFuelIndex
  (params (Index :type Integer))
  (bind _parentchestref (Variables|General|GetParentChestRef))
  (bind _cookingmodule (Variables|/Game/AdvancedInventory/Blueprints/Chests/BP_0_Chest_Master.BP_0_Chest_Master_C|GetCookingModule _parentchestref))
  (bind (_amountofcookingslots _amountoffuelbars _amountoffuelslotsperbar) (Utilities|Struct|BreakS_ChestCookingModule _cookingmodule))
  ;[1 1 1] Check if input index is index in fuel section
  (return (and (>= Index _amountofcookingslots) (< Index (+ _amountofcookingslots (* _amountoffuelbars _amountoffuelslotsperbar))))))

(fn GetChestItemDatabyIndex
  (params (Index :type Integer))
  ;[1 1 1] get item data of specific chest slot
  (return (CallFunction|StringtoItemData (Utilities|Array|Get(acopy) (Variables|/Game/AdvancedInventory/Blueprints/Chests/BP_0_Chest_Master.BP_0_Chest_Master_C|GetItemString_AllSlots (Variables|General|GetParentChestRef)) Index))))

(fn UpdateChestItemDatabyIndex
  (params (Index :type Integer) (itemData :type S%20Item%20Data%20Structure))
  ;[1 1 1] Update specific chest item data
  (Utilities|Array|SetArrayElem (Variables|/Game/AdvancedInventory/Blueprints/Chests/BP_0_Chest_Master.BP_0_Chest_Master_C|GetItemString_AllSlots (Variables|General|GetParentChestRef)) Index (CallFunction|ItemDatatoString itemData)))

(fn StopCooking
  ;[1 1 1] Completely stop cooking and reset cooking arrays
  (Utilities|Time|ClearandInvalidateTimerbyHandle (Variables|General|GetCookTimer))
  (Default|CallOnCookingTurnedon (Variables|General|GetParentChestRef) false)
  (Variables|General|SetbCooking false)
  (for _index (range 0 (- (Utilities|Array|Length (Variables|CookingSlots|GetSecondsCookedArray)) 1))
    (Utilities|Array|SetArrayElem (Variables|CookingSlots|GetSecondsCookedArray) _index 0.0)
    (Utilities|Array|SetArrayElem (Variables|CookingSlots|GetSecondsToCookArray) _index 0.0)))

(fn UpdateCookingProgress
  (params (Percent :type Array%20of%20Integers) (TurnOffCampfire :type Boolean))
  ;[1 1 1] Reduce fuel and update percent of cooking progress in UI
  (LocalVariables|SetTurnOff TurnOffCampfire)
  (Variables|General|SetFuel (- (Variables|General|GetFuel) (Variables|General|GetCookInterval)))
  (if (<= (Variables|General|GetFuel) 0.0)
    (bind (_found _fuelamount _itemindex) (Updating|FindFuelItemandUpdate))
    (if _found
      (Variables|General|SetFuel _fuelamount)
      (Updating|UpdateCookingUIforAllPlayers (Utilities|Struct|MakeS_ChestCookingUpdateData (select (or (<= (Variables|General|GetFuel) 0.0) (LocalVariables|GetTurnOff)) (Other|AllCookingSlotstoZero) Percent) true _itemindex)))
    (else
      (Updating|UpdateCookingUIforAllPlayers (Utilities|Struct|MakeS_ChestCookingUpdateData (select (or (<= (Variables|General|GetFuel) 0.0) (LocalVariables|GetTurnOff)) (Other|AllCookingSlotstoZero) Percent)))))
  ;[1 1 1] Check to stop cooking
  (if (or (<= (Variables|General|GetFuel) 0.0) (LocalVariables|GetTurnOff))
    (General|StopCooking)
    (Updating|UpdateCookingUIforAllPlayers (Utilities|Struct|MakeS_ChestCookingUpdateData (Other|AllCookingSlotstoZero)))))

(fn UpdateCookingUIforAllPlayers
  (params (UpdateData :type S%20Chest%20Cooking%20Update%20Data%20Structure))
  ;[1 1 1] Update cooking data for all players that are currently interacting with this chest
  (LocalVariables|SetL_UpdateData UpdateData)
  (for _array_element (Variables|/Game/AdvancedInventory/Blueprints/Components/AC_InventoryGameMode_Component.AC_InventoryGameMode_Component_C|GetAllPCsAndComponents (Variables|Default|GetGameModeComponentRef))
    (if (== (Variables|/Game/AdvancedInventory/Blueprints/Components/AC_InventoryPC_Component.AC_InventoryPC_Component_C|GetCurrentChestRefServer (.PC_Component (Utilities|Struct|BreakS_PCsAndComponents _array_element))) (Variables|General|GetParentChestRef))
      (Default|UpdateOwnCookingUI (.PC_Component (Utilities|Struct|BreakS_PCsAndComponents _array_element)) (LocalVariables|GetL_UpdateData)))))

(fn GenerateUniqueID
  (params (ItemID :type Name))
  ;[1 1 1] Generates unique ID for item that is important for chest replication
  (return (Utilities|String|Append (Utilities|String|ToString(Name) ItemID) "_" (Utilities|String|ToString(Integer) (Math|Random|RandomIntegerinRange 10 9999)) (Utilities|Select :Index (Math|Random|RandomIntegerinRange 0 8) :Option%200 "A" :Option%201 "B" :Option%202 "C" :Option%203 "D" :Option%204 "E" :Option%205 "F" :Option%206 "H" :Option%207 "I" :Option%208 "J"))))

(fn GetFirstContentSlotIndex
  (bind _parentchestref (Variables|General|GetParentChestRef))
  (bind _cookingmodule (Variables|/Game/AdvancedInventory/Blueprints/Chests/BP_0_Chest_Master.BP_0_Chest_Master_C|GetCookingModule _parentchestref))
  (bind (_amountofcookingslots _amountoffuelbars _amountoffuelslotsperbar) (Utilities|Struct|BreakS_ChestCookingModule _cookingmodule))
  ;[1 1 1] get index of first content slot
  (return (+ _amountofcookingslots (* _amountoffuelbars _amountoffuelslotsperbar))))