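; Server-side component for BP_0_Vendor_Master actors that lets players list and buy products in a shared shop.
; Listing stamps seller ID and name, then adds the product to the seller's current vendor.
; Buying re-resolves stale indices by ProductID, checks money and stock, grants the item, and pays the seller directly or via cloud user ID.
; Both refresh the UI of players viewing that vendor through the GameMode component's player list.
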(event EventBeginPlay
  ;[1 1 1] Begin Play
  (CallFunction|SetUp))

(fn SetUp
  (Utilities|IsValid (Game|GetGameMode) ; Set up only happens on server
    (:Is%20Valid
      ;[1 1 1] set up references
      (bind _asbp_0_vendor_master (Utilities|Casting|CastToBP_0_Vendor_Master (Components|GetOwner)))
      (Variables|Default|SetVendorRef _asbp_0_vendor_master)
      (Variables|Default|SetGameModeComponentRef (Actor|GetComponentbyClass (Game|GetGameMode) "/Game/AdvancedInventory/Blueprints/Components/AC_InventoryGameMode_Component.AC_InventoryGameMode_Component_C")))))

(fn AddProductforSale
  (params (product%20data :type S%20Vendor%20Product%20Structure))
  ;[1 1 1] Setup local variable(s)
  (bind _output_get (LocalVariables|SetProductData product%20data))
  ;[1 1 1] Set up vendor owner
  (Utilities|Struct|SetmembersinS_VendorProduct (LocalVariables|GetProductData) (Variables|/Game/AdvancedInventory/Blueprints/Components/AC_InventoryPC_Component.AC_InventoryPC_Component_C|GetCustomUserID_ForCloudMoneyHandling (CallFunction|GetInventoryPCComponent (Utilities|Struct|BreakS_VendorProduct _output_get))) (Utilities|Text|ToText(String) (PlayerState|GetPlayerName (Variables|/Script/Engine.Controller|GetPlayerState (Utilities|Struct|BreakS_VendorProduct _output_get)))))
  ;[1 1 1] Add product to vendor actor
  (Default|AddProduct (Variables|/Game/AdvancedInventory/Blueprints/Components/AC_InventoryPC_Component.AC_InventoryPC_Component_C|GetCurrentVendorRefServer (CallFunction|GetInventoryPCComponent (Utilities|Struct|BreakS_VendorProduct _output_get))) (LocalVariables|GetProductData))
  ;[1 1 1] Update Vendor UI on all players who are currently interacting with the same shop
  (for _array_element (Variables|/Game/AdvancedInventory/Blueprints/Components/AC_InventoryGameMode_Component.AC_InventoryGameMode_Component_C|GetAllPCsAndComponents (Variables|Default|GetGameModeComponentRef))
    (if (== (Variables|/Game/AdvancedInventory/Blueprints/Components/AC_InventoryPC_Component.AC_InventoryPC_Component_C|GetCurrentVendorRefServer (CallFunction|GetInventoryPCComponent (Utilities|Struct|BreakS_VendorProduct (LocalVariables|GetProductData)))) (Variables|/Game/AdvancedInventory/Blueprints/Components/AC_InventoryPC_Component.AC_InventoryPC_Component_C|GetCurrentVendorRefServer (Utilities|Struct|BreakS_PCsAndComponents _array_element)))
      (Default|UpdateVendorUIClient (Utilities|Struct|BreakS_PCsAndComponents _array_element) (Variables|/Game/AdvancedInventory/Blueprints/Components/AC_InventoryPC_Component.AC_InventoryPC_Component_C|GetCurrentVendorRefServer (Utilities|Struct|BreakS_PCsAndComponents _array_element)) (Variables|/Game/AdvancedInventory/Blueprints/Vendors/BP_0_Vendor_Master.BP_0_Vendor_Master_C|GetProducts (Variables|/Game/AdvancedInventory/Blueprints/Components/AC_InventoryPC_Component.AC_InventoryPC_Component_C|GetCurrentVendorRefServer (Utilities|Struct|BreakS_PCsAndComponents _array_element)))))))

(fn BuyProduct
  (params (buyData :type S%20Buy%20Vendor%20Product%20Structure))
  ;[1 1 1] Save values to local variables
  (bind _output_get (LocalVariables|SetBuyProductData buyData))
  (LocalVariables|SetPC_Component (CallFunction|GetInventoryPCComponent (Utilities|Struct|BreakS_BuyVendorProduct _output_get)))
  (Utilities|FlowControl|Sequence
    (:then_0
      ;[1 1 1] check if requested index exists
      (if (< (Utilities|Struct|BreakS_BuyVendorProduct (LocalVariables|GetBuyProductData)) (Utilities|Array|Length (Variables|/Game/AdvancedInventory/Blueprints/Vendors/BP_0_Vendor_Master.BP_0_Vendor_Master_C|GetProducts (Variables|Default|GetVendorRef))))
        ;[1 1 1] Get actual product index (players might be outdated)
        (if (Utilities|Enum|Equal(Enum) (Utilities|Struct|BreakS_VendorProduct (Utilities|Array|Get(acopy) (Variables|/Game/AdvancedInventory/Blueprints/Vendors/BP_0_Vendor_Master.BP_0_Vendor_Master_C|GetProducts (Variables|Default|GetVendorRef)) (Utilities|Struct|BreakS_BuyVendorProduct (LocalVariables|GetBuyProductData)))) (Utilities|Struct|BreakS_BuyVendorProduct (LocalVariables|GetBuyProductData)))
          (LocalVariables|SetActualProductIndex (Utilities|Struct|BreakS_BuyVendorProduct (LocalVariables|GetBuyProductData)))
          ;[1 1 1] Check if player has enough money
          (if (>= (Variables|/Game/AdvancedInventory/Blueprints/Components/AC_InventoryPC_Component.AC_InventoryPC_Component_C|GetMoney (LocalVariables|GetPC_Component)) (Utilities|Struct|BreakS_VendorProduct (Utilities|Array|Get(acopy) (Variables|/Game/AdvancedInventory/Blueprints/Vendors/BP_0_Vendor_Master.BP_0_Vendor_Master_C|GetProducts (Variables|Default|GetVendorRef)) (LocalVariables|GetActualProductIndex)))) :!label _label
            ;[1 1 1] Add product to buying player & remove money
            (if (> (Utilities|Struct|BreakS_VendorProduct (Utilities|Array|Get(acopy) (Variables|/Game/AdvancedInventory/Blueprints/Vendors/BP_0_Vendor_Master.BP_0_Vendor_Master_C|GetProducts (Variables|Default|GetVendorRef)) (LocalVariables|GetActualProductIndex))) 0)
              (bind _output_get_2 (LocalVariables|SetRemoveProduct (<= (- (Utilities|Struct|BreakS_VendorProduct (Utilities|Array|Get(acopy) (Variables|/Game/AdvancedInventory/Blueprints/Vendors/BP_0_Vendor_Master.BP_0_Vendor_Master_C|GetProducts (Variables|Default|GetVendorRef)) (LocalVariables|GetActualProductIndex))) 1) 0)))
              (if _output_get_2
                (Utilities|Struct|SetmembersinS_VendorProduct (Utilities|Array|Get(acopy) (Variables|/Game/AdvancedInventory/Blueprints/Vendors/BP_0_Vendor_Master.BP_0_Vendor_Master_C|GetProducts (Variables|Default|GetVendorRef)) (LocalVariables|GetActualProductIndex)))
                (else
                  (Utilities|Struct|SetmembersinS_VendorProduct (Utilities|Array|Get(acopy) (Variables|/Game/AdvancedInventory/Blueprints/Vendors/BP_0_Vendor_Master.BP_0_Vendor_Master_C|GetProducts (Variables|Default|GetVendorRef)) (LocalVariables|GetActualProductIndex)) (- (Utilities|Struct|BreakS_VendorProduct (Utilities|Array|Get(acopy) (Variables|/Game/AdvancedInventory/Blueprints/Vendors/BP_0_Vendor_Master.BP_0_Vendor_Master_C|GetProducts (Variables|Default|GetVendorRef)) (LocalVariables|GetActualProductIndex))) 1))))
              (Default|AddItemtoPlayeronOwningPlayer (LocalVariables|GetPC_Component) (CallFunction|ItemDatatoString (.itemData (Utilities|Struct|BreakS_VendorProduct (Utilities|Array|Get(acopy) (Variables|/Game/AdvancedInventory/Blueprints/Vendors/BP_0_Vendor_Master.BP_0_Vendor_Master_C|GetProducts (Variables|Default|GetVendorRef)) (LocalVariables|GetActualProductIndex))))) false)
              (Default|AddMoneyonServerandUpdateUI (LocalVariables|GetPC_Component) (* (.Price (Utilities|Struct|BreakS_VendorProduct (Utilities|Array|Get(acopy) (Variables|/Game/AdvancedInventory/Blueprints/Vendors/BP_0_Vendor_Master.BP_0_Vendor_Master_C|GetProducts (Variables|Default|GetVendorRef)) (LocalVariables|GetActualProductIndex)))) -1))
              ;[1 1 1] Add money to owner (if valid player)
              ; or to CustomUserID (cloud server)
              (if (Variables|Default|GetbUseCustomUserIDForMoneyHandlingOnCloud)
                (Default|AddMoneytoCustomID (Variables|Default|GetGameModeComponentRef) (.Price (Utilities|Struct|BreakS_VendorProduct (Utilities|Array|Get(acopy) (Variables|/Game/AdvancedInventory/Blueprints/Vendors/BP_0_Vendor_Master.BP_0_Vendor_Master_C|GetProducts (Variables|Default|GetVendorRef)) (LocalVariables|GetActualProductIndex)))) (.CustomOwnerID (Utilities|Struct|BreakS_VendorProduct (Utilities|Array|Get(acopy) (Variables|/Game/AdvancedInventory/Blueprints/Vendors/BP_0_Vendor_Master.BP_0_Vendor_Master_C|GetProducts (Variables|Default|GetVendorRef)) (LocalVariables|GetActualProductIndex)))))
                (else
                  (Utilities|IsValid (.OwnerPC (Utilities|Struct|BreakS_VendorProduct (Utilities|Array|Get(acopy) (Variables|/Game/AdvancedInventory/Blueprints/Vendors/BP_0_Vendor_Master.BP_0_Vendor_Master_C|GetProducts (Variables|Default|GetVendorRef)) (LocalVariables|GetActualProductIndex))))
                    (:Is%20Valid
                      (Default|AddMoneyonServerandUpdateUI (CallFunction|GetInventoryPCComponent (.OwnerPC (Utilities|Struct|BreakS_VendorProduct (Utilities|Array|Get(acopy) (Variables|/Game/AdvancedInventory/Blueprints/Vendors/BP_0_Vendor_Master.BP_0_Vendor_Master_C|GetProducts (Variables|Default|GetVendorRef)) (LocalVariables|GetActualProductIndex))))) (.Price (Utilities|Struct|BreakS_VendorProduct (Utilities|Array|Get(acopy) (Variables|/Game/AdvancedInventory/Blueprints/Vendors/BP_0_Vendor_Master.BP_0_Vendor_Master_C|GetProducts (Variables|Default|GetVendorRef)) (LocalVariables|GetActualProductIndex))))))
                    (:Is%20Not%20Valid
                      _))))
              ;[1 1 1] Remove product from array if quantity is smaller than 1
              (if (LocalVariables|GetRemoveProduct)
                (Utilities|Array|RemoveIndex (Variables|/Game/AdvancedInventory/Blueprints/Vendors/BP_0_Vendor_Master.BP_0_Vendor_Master_C|GetProducts (Variables|Default|GetVendorRef)) (LocalVariables|GetActualProductIndex)))
              ;[1 1 1] Update Vendor UI for all players that currently have the same vendor opened
              (for _array_element (Variables|/Game/AdvancedInventory/Blueprints/Components/AC_InventoryGameMode_Component.AC_InventoryGameMode_Component_C|GetAllPCsAndComponents (Variables|Default|GetGameModeComponentRef))
                (if (== (Variables|Default|GetVendorRef) (Variables|/Game/AdvancedInventory/Blueprints/Components/AC_InventoryPC_Component.AC_InventoryPC_Component_C|GetCurrentVendorRefServer (Utilities|Struct|BreakS_PCsAndComponents _array_element)))
                  (Default|UpdateVendorUIClient (Utilities|Struct|BreakS_PCsAndComponents _array_element) (Variables|/Game/AdvancedInventory/Blueprints/Components/AC_InventoryPC_Component.AC_InventoryPC_Component_C|GetCurrentVendorRefServer (Utilities|Struct|BreakS_PCsAndComponents _array_element)) (Variables|/Game/AdvancedInventory/Blueprints/Vendors/BP_0_Vendor_Master.BP_0_Vendor_Master_C|GetProducts (Variables|/Game/AdvancedInventory/Blueprints/Components/AC_InventoryPC_Component.AC_InventoryPC_Component_C|GetCurrentVendorRefServer (Utilities|Struct|BreakS_PCsAndComponents _array_element))))))))
          (else
            (bind _output_get_3 (LocalVariables|SetActualProductIndex (CallFunction|FindProductIndexbyProductID (Variables|/Game/AdvancedInventory/Blueprints/Vendors/BP_0_Vendor_Master.BP_0_Vendor_Master_C|GetProducts (Variables|Default|GetVendorRef)) (Utilities|Struct|BreakS_BuyVendorProduct (LocalVariables|GetBuyProductData)))))
            (if (!= _output_get_3 -1)
              (goto _label))))))
    (:then_1
      (Default|HideVendorLoadingBox (LocalVariables|GetPC_Component)))))

(fn FindProductIndexbyProductID
  (params (Products :type Array%20of%20S%20Vendor%20Product%20Structures) (ProductID :type String))
  ;[1 1 1] Seaching whole product list for product with specific ID (only happens if rquested index element had no matching ProductID with requested ProdoductID)
  (for (_array_element _array_index) Products
    (if (Utilities|Enum|Equal(Enum) (Utilities|Struct|BreakS_VendorProduct _array_element) ProductID)
      (return _array_index)))
  (return -1))