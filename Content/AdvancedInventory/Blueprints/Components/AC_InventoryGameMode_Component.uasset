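; Game mode component of the inventory system that handles item pickups and tracks connected players.
; Login and logout maintain a list of player controllers with their inventory components.
; Pickups hand dropped item data to the player's component as a string; ground-list pickups take a clamped amount, destroy emptied actors and refresh every player's ground list.
; AddMoneyToCustomID is an empty placeholder for crediting money on a cloud server.
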(fn PickUpGroundListItem
  (params (PC :type Player%20Controller%20Object%20Reference) (ItemActor :type Actor%20Object%20Reference) (Amount :type Integer))
  ;[1 1 1] Set up
  (bind _output_get (LocalVariables|SetItem ItemActor))
  (Utilities|IsValid _output_get
    (:Is%20Valid
      (LocalVariables|SetRequestedAmount Amount)
      (LocalVariables|SetPlayerController PC)
      ;[1 1 1] adds requested item to players inventory (if possible) and destroy item if the remaining amount would become 0
      (bind _asbp_drop_item_actor (Utilities|Casting|CastToBP_DropItemActor (LocalVariables|GetItem)))
      (LocalVariables|SetItemDataCopy (Variables|/Game/AdvancedInventory/Blueprints/General/BP_DropItemActor.BP_DropItemActor_C|GetItemDataNew _asbp_drop_item_actor))
      (if (<= (- (Utilities|Struct|BreakS_ItemData (Variables|/Game/AdvancedInventory/Blueprints/General/BP_DropItemActor.BP_DropItemActor_C|GetItemDataNew _asbp_drop_item_actor)) (Math|Integer|Clamp(Integer) (LocalVariables|GetRequestedAmount) 1 (Utilities|Struct|BreakS_ItemData (Variables|/Game/AdvancedInventory/Blueprints/General/BP_DropItemActor.BP_DropItemActor_C|GetItemDataNew _asbp_drop_item_actor)))) 0)
        (Default|AddItemtoPlayeronOwningPlayer (CallFunction|GetInventoryPCComponent (LocalVariables|GetPlayerController)) (CallFunction|ItemDatatoString (LocalVariables|GetItemDataCopy)) false)
        (Actor|DestroyActor (LocalVariables|GetItem))
        (else
          (Utilities|Struct|SetmembersinS_ItemData (LocalVariables|GetItemDataCopy) (Math|Integer|Clamp(Integer) (LocalVariables|GetRequestedAmount) 1 (Utilities|Struct|BreakS_ItemData (Variables|/Game/AdvancedInventory/Blueprints/General/BP_DropItemActor.BP_DropItemActor_C|GetItemDataNew _asbp_drop_item_actor))))
          (bind _structout (Utilities|Struct|SetmembersinS_ItemData (Variables|/Game/AdvancedInventory/Blueprints/General/BP_DropItemActor.BP_DropItemActor_C|GetItemDataNew _asbp_drop_item_actor) (- (Utilities|Struct|BreakS_ItemData (Variables|/Game/AdvancedInventory/Blueprints/General/BP_DropItemActor.BP_DropItemActor_C|GetItemDataNew _asbp_drop_item_actor)) (Math|Integer|Clamp(Integer) (LocalVariables|GetRequestedAmount) 1 (Utilities|Struct|BreakS_ItemData (Variables|/Game/AdvancedInventory/Blueprints/General/BP_DropItemActor.BP_DropItemActor_C|GetItemDataNew _asbp_drop_item_actor))))))
          (Variables|/Game/AdvancedInventory/Blueprints/General/BP_DropItemActor.BP_DropItemActor_C|SetItemDataNew _asbp_drop_item_actor _structout)
          (Default|AddItemtoPlayeronOwningPlayer (CallFunction|GetInventoryPCComponent (LocalVariables|GetPlayerController)) (CallFunction|ItemDatatoString (LocalVariables|GetItemDataCopy)) false)))
      ;[1 1 1] Update ground list for everyone
      (for _array_element (Variables|Default|GetAllPCsAndComponents)
        (Default|UpdateGroundItemListPC (Utilities|Struct|BreakS_PCsAndComponents _array_element))))))

(fn PCLogin
  (params (PC :type Player%20Controller%20Object%20Reference))
  ;[1 1 1] Adding player
  (Utilities|IsValid PC
    (:Is%20Valid
      (Utilities|Array|Add (Variables|Default|GetAllPCsAndComponents) (Utilities|Struct|MakeS_PCsAndComponents PC (CallFunction|GetInventoryPCComponent PC))))))

(fn PCLogout
  (params (PC :type Controller%20Object%20Reference))
  ;[1 1 1] Removing player
  (bind _asplayer_controller (Utilities|Casting|CastToPlayerController PC))
  (for (_array_element _array_index) (Variables|Default|GetAllPCsAndComponents)
    (if (== (Utilities|Struct|BreakS_PCsAndComponents _array_element) _asplayer_controller)
      (Utilities|Array|RemoveIndex (Variables|Default|GetAllPCsAndComponents) _array_index)
      (return))))

(fn PickUpItem
  (params (PC_Component :type AC%20Inventory%20PC%20Component%20Object%20Reference) (ItemActor :type Actor%20Object%20Reference))
  ;[1 1 1] check if item is still valid, if so transfer it to the inventory of the requesting player and destroy the actor
  (Utilities|IsValid ItemActor
    (:Is%20Valid
      (bind _asbp_drop_item_actor (Utilities|Casting|CastToBP_DropItemActor ItemActor))
      (Default|AddItemtoPlayeronOwningPlayer PC_Component (CallFunction|ItemDatatoString (Variables|/Game/AdvancedInventory/Blueprints/General/BP_DropItemActor.BP_DropItemActor_C|GetItemDataNew _asbp_drop_item_actor)) false)
      (Actor|DestroyActor ItemActor))))

(fn AddMoneytoCustomID
  (params (MoneyToAdd :type Integer) (CustomUserID :type String))
  ;[1 1 1] Could execute here a function to add money on a cloud server
)