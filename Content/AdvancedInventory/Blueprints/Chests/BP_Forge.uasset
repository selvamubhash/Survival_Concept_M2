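; BP_Forge is a forge in the inventory system's chest family that cooks through a CookingComponent and shows fire while running.
; On BeginPlay, only the authority binds the check-cooking and cooking-turned-on events.
; Cooking checks are forwarded to the component, while on/off changes set the replicated TurnedOn flag.
; Its OnRep toggles the PFireForge effect to match.
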(event Custom|CheckCooking
  (params (ResetSecondsCooked :type Boolean) (ResetSlot :type Integer))
  ;[1 1 1] Only server relevant bindings
  (Default|CheckCooking (Variables|Default|GetCookingComponent) ResetSecondsCooked ResetSlot))

(event Custom|OnCookingTurnendOnOff_Event
  (params (TurnedOn :type Boolean))
  ;[1 1 1] Only server relevant bindings
  (Variables|Default|SetTurnedOn TurnedOn))

(event EventBeginPlay
  (|CallParentFunction)
  ;[1 1 1] Only server relevant bindings
  (Networking|SwitchHasAuthority
    (:Authority
      (EventDispatchers|BindEventtoOnCheckCooking (delegate Custom|CheckCooking))
      (EventDispatchers|AssignOnCookingTurnedon (delegate Custom|OnCookingTurnendOnOff_Event)))))

(fn ConstructionScript
  (|CallParentFunction))

(fn OnRepTurnedon
  (Components|Activation|SetActive (Variables|Default|GetP_FireForge) (Variables|Default|GetTurnedOn) false))