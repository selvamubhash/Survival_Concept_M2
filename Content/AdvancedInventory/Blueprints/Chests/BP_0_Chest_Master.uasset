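; Master chest Blueprint for the inventory system, configurable as normal storage, cooking, dead-player loot or loot chest.
; On BeginPlay the server sizes slot arrays from the enabled module, sets filters, adds a cooking component if needed and rolls randomized starting items.
; Slot contents are stored as item strings with visibility flags.
; Loot chests instead queue items and, once opened, launch them one by one as physical drops on a timer.
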(event Custom|ToggleFocus
  (params (Focus :type Boolean))
  ;[1 1 1] ToggleFocus and Call dispatcher event to notify child chest
  (Rendering|SetRenderCustomDepth (Variables|Default|GetchestModel) Focus)
  (Default|CallOnFocus Focus))

(event Custom|DropAllItems
  (params (pc :type Player%20Controller%20Object%20Reference))
  ;[1 1 1] Loot Chest: Call drop if chest is unopened loot chest
  (if (not (Variables|LootChest|GetbLootChestOpened))
    (Variables|LootChest|SetbLootChestOpened true)
    (LootChest&StartingItems|StartDropping)))

(event EventBeginPlay
  ;[1 1 1] Event Begin Play and set up
  (SetUp|SetUp))

(fn ConstructionScript)

(fn MakeRandomDirection
  ;[1 1 1] generate random xy vector scaled to a random length (RadiusMin&RadiusMax)
  (bind _output_get (LocalVariables|SetL_RandomVector (Math|Random|RandomUnitVector)))
  (bind _output_get_2 (LocalVariables|SetL_RandomVector (* (Math|Vector|MakeVector (.X (Math|Vector|BreakVector _output_get)) (.Y (Math|Vector|BreakVector _output_get)) 0.0) (/ (Math|Conversions|ToFloat(Integer) (Math|Random|RandomIntegerinRange (LocalVariables|GetRadiusMin) (LocalVariables|GetRadiusMax))) (Math|Vector|VectorLength (Math|Vector|MakeVector (.X (Math|Vector|BreakVector _output_get)) (.Y (Math|Vector|BreakVector _output_get)) 0.0))))))
  ;[1 1 1] Add Z velocity
  (bind _output_get_3 (LocalVariables|SetL_RandomVector (Math|Vector|MakeVector (.X (Math|Vector|BreakVector _output_get_2)) (.Y (Math|Vector|BreakVector _output_get_2)) 7.5e+02)))
  (return _output_get_3))

(fn SetUp
  (CallFunction|SetUpInteractDuration)
  (Components|Sphere|SetSphereRadius (Variables|Default|GetInteractionFalloffSphere) (Variables|SetUp|GetInteractionFallOffRadius) true)
  (Networking|SwitchHasAuthority
    (:Authority
      (SetUp|CheckforCookingComponent)
      ;[1 1 1] Loop to set up essential arrays fitting to chest slot amount
      (for _index (range 1 (SetUp|CalculateChestSlotsAmount))
        (Utilities|Array|Add (Variables|StartingItems|GetShuffle) (- _index 1))
        (Utilities|Array|Add (Variables|General|GetVisibility_AllSlots) false)
        (Utilities|Array|Add (Variables|General|GetItemString_AllSlots) ""))
      ;[1 1 1] Custom filter set up for normal chests
      (CallFunction|SetUpItemFiltersArrayandSpecialSlotsNormalChest)
      ;[1 1 1] Custom filter set up for cooking chests
      (SetUp|SetUpItemFiltersArrayandSpecialSlotsCookingModule)
      ;[1 1 1] Set up starting items on server
      (Networking|SwitchHasAuthority
        (:Authority
          (if (and (Utilities|Struct|BreakS_ChestStartingItemsModule (Variables|Modules|GetStartingItemsModule)) (not (Utilities|Struct|BreakS_ChestCookingModule (Variables|Modules|GetCookingModule))))
            (LootChest&StartingItems|AddStartingItems)))))))

(fn CheckforCookingComponent
  ;[1 1 1] Add automatically cooking component to chest if module is enabled
  (if (Utilities|Struct|BreakS_ChestCookingModule (Variables|Modules|GetCookingModule))
    (bind _returnvalue (AddComponent|AddACChestCookingComponent))
    (Variables|Default|SetCookingComponent _returnvalue)))

(fn CalculateChestSlotsAmount
  (bind _cookingmodule (Variables|Modules|GetCookingModule))
  (bind _lootdeadplayermodule (Variables|Modules|GetLootDeadPlayerModule))
  (bind _chestmodule (Variables|Modules|GetChestModule))
  (bind (_enabled _amountofbars _amountofslotsperbar) (Utilities|Struct|BreakS_ChestModule _chestmodule))
  (bind (_enabled_2 _amountofcookingslots _amountoffuelbars _amountoffuelslotsperbar _amountofcontentbars _amountofcontentslotsperbar) (Utilities|Struct|BreakS_ChestCookingModule _cookingmodule))
  (bind (_enabled_3 _inventoryamountofbars _inventoryamountofslotsperbar _equipamountofbars _equipamountofslotsperbar) (Utilities|Struct|BreakS_ChestLootDeadPlayerModule _lootdeadplayermodule))
  ;[1 1 1] normal chest
  (if _enabled
    (return (* _amountofbars _amountofslotsperbar))
    (else
      ;[1 1 1] cooking chest
      (if _enabled_2
        (return (+ _amountofcookingslots (* _amountoffuelbars _amountoffuelslotsperbar) (* _amountofcontentbars _amountofcontentslotsperbar)))
        (else
          ;[1 1 1] loot dead body chest
          (if _enabled_3
            (return (+ (* _inventoryamountofbars _inventoryamountofslotsperbar) (* _equipamountofbars _equipamountofslotsperbar)))))))))

(fn AddStartingItems
  (bind _startingitemsmodule (Variables|Modules|GetStartingItemsModule))
  (bind (_islootchest _randomsorting) (Utilities|Struct|BreakS_ChestStartingItemsModule _startingitemsmodule))
  ;[1 1 1] Create sorting array and start loop
  (if (and _islootchest _randomsorting)
    (Utilities|Array|Shuffle (Utilities|Struct|BreakS_ChestStartingItemsModule (Variables|Modules|GetStartingItemsModule)))
    (else
      (for _index (range 0 (Utilities|Array|LastIndex (Variables|General|GetVisibility_AllSlots)))
        (Utilities|Array|Add (LocalVariables|GetSorting) _index))))
  (if (Utilities|Struct|BreakS_ChestStartingItemsModule (Variables|Modules|GetStartingItemsModule))
    (Utilities|Array|Shuffle (LocalVariables|GetSorting)))
  (for (_array_element _array_index) (Utilities|Struct|BreakS_ChestStartingItemsModule (Variables|Modules|GetStartingItemsModule))
    (LocalVariables|SetSI_Element _array_element)
    (LocalVariables|SetSI_Index _array_index)
    ;[1 1 1] Create item data and check if item should appear
    (bind (_out_row _found) (CallFunction|GetItemDatabyID (Utilities|Struct|BreakDataTableRowHandle (Utilities|Struct|BreakS_ChestStartingItem (LocalVariables|GetSI_Element)))))
    (if _found
      (bind _output_get (LocalVariables|SetItemToAdd _out_row))
      (Utilities|Struct|SetmembersinS_AdditionalGeneralData (.AdditionalGeneralData (Utilities|Struct|BreakS_ItemData _output_get)) (LootChest&StartingItems|GenerateUniqueID (.ID (Utilities|Struct|BreakS_ItemData _output_get))))
      (bind _output_get_2 (LocalVariables|SetPercentAppear (Math|Random|RandomIntegerinRange 0 100)))
      (if (>= (Utilities|Struct|BreakS_ChestStartingItem (LocalVariables|GetSI_Element)) _output_get_2)
        ;[1 1 1] Generate random item amount
        (bind _output_get_3 (LocalVariables|SetStartingItemAmount (Math|Random|RandomIntegerinRange (.AmountMin (Utilities|Struct|BreakS_ChestStartingItem (LocalVariables|GetSI_Element))) (.AmountMax (Utilities|Struct|BreakS_ChestStartingItem (LocalVariables|GetSI_Element))))))
        (if (> _output_get_3 0)
          ;[1 1 1] Set item amount
          (Utilities|Struct|SetmembersinS_ItemData (LocalVariables|GetItemToAdd) (select (.Stackable (Utilities|Struct|BreakS_AdditionalGeneralData (Utilities|Struct|BreakS_ItemData (LocalVariables|GetItemToAdd)))) (select (> (LocalVariables|GetStartingItemAmount) (.MaxStackSize (Utilities|Struct|BreakS_AdditionalGeneralData (Utilities|Struct|BreakS_ItemData (LocalVariables|GetItemToAdd))))) (.MaxStackSize (Utilities|Struct|BreakS_AdditionalGeneralData (Utilities|Struct|BreakS_ItemData (LocalVariables|GetItemToAdd)))) (LocalVariables|GetStartingItemAmount)) 1))
          ;[1 1 1] Check if durability is enabled
          (if (Utilities|Struct|BreakS_Durability (Utilities|Struct|BreakS_ItemData (LocalVariables|GetItemToAdd)))
            ;[1 1 1] Random durability
            (bind _output_get_4 (LocalVariables|SetRandomDurability (Math|Float|Clamp(Float) (Math|Random|RandomFloatinRange (.X (Math|Vector2D|BreakVector2D (.DurabilityRangePercentage_0_to_1 (Utilities|Struct|BreakS_ChestStartingItem (LocalVariables|GetSI_Element))))) (.Y (Math|Vector2D|BreakVector2D (.DurabilityRangePercentage_0_to_1 (Utilities|Struct|BreakS_ChestStartingItem (LocalVariables|GetSI_Element)))))))))
            (if (> _output_get_4 0.0)
              (Utilities|Struct|SetmembersinS_Durability (Utilities|Struct|BreakS_ItemData (LocalVariables|GetItemToAdd)) (* (LocalVariables|GetRandomDurability) (Utilities|Struct|BreakS_Durability (Utilities|Struct|BreakS_ItemData (LocalVariables|GetItemToAdd)))))
              ;[1 1 1] Add ItemString and visibility
              (Utilities|Array|Add (Variables|StartingItems|GetNewStartingItems) (LocalVariables|GetItemToAdd) :!label _label)
              (if (not (Utilities|Struct|BreakS_ChestStartingItemsModule (Variables|Modules|GetStartingItemsModule)))
                (Utilities|Array|SetArrayElem (Variables|General|GetItemString_AllSlots) (Utilities|Array|Get(acopy) (LocalVariables|GetSorting) (LocalVariables|GetSI_Index)) (CallFunction|ItemDatatoString (LocalVariables|GetItemToAdd)))
                (Utilities|Array|SetArrayElem (Variables|General|GetVisibility_AllSlots) (Utilities|Array|Get(acopy) (LocalVariables|GetSorting) (LocalVariables|GetSI_Index)) true)))
            (else
              (goto _label))))))))

(fn OnRepIsLootboxOpened?)

(fn StartDropping
  ;[1 1 1] Loot Chest: Create a loop that drops all items
  (if (> (Utilities|Array|Length (Variables|StartingItems|GetNewStartingItems)) 0)
    (Utilities|Time|SetTimerbyFunctionName 0 "DropNextLootBoxItemInRow" (Variables|LootChest|GetTimeBetweenItemDropping))))

(fn DropNextLootBoxIteminRow
  (bind _newstartingitems (Variables|StartingItems|GetNewStartingItems))
  (bind _output (Utilities|Array|Get(acopy) _newstartingitems))
  ;[1 1 1] Spawn and set up item actor
  (bind _returnvalue (Game|SpawnActorfromClass "/Game/AdvancedInventory/Blueprints/General/BP_DropItemActor.BP_DropItemActor_C" (Math|Transform|MakeTransform (Transformation|GetWorldLocation (Variables|Default|GetLootChestSpawnLocation))) "Undefined" "OverrideRootScale" 0 (Utilities|Struct|MakeS_SpawnItemSettings false "(DataTable=None,RowName=\"\")") 1 0.0 false 0))
  (Utilities|Struct|SetmembersinS_AdditionalGeneralData (Utilities|Struct|BreakS_ItemData _output))
  (Default|Update _returnvalue _output)
  (bind _output_get (Variables|LootChest|SetRandomDirection (LootChest&StartingItems|MakeRandomDirection)))
  (Variables|/Script/Engine.MovementComponent|SetVelocity (Variables|/Game/AdvancedInventory/Blueprints/General/BP_DropItemActor.BP_DropItemActor_C|GetProjectileMovement _returnvalue) _output_get)
  ;[1 1 1] Remove spawned item from queue and repeat process
  (Utilities|Array|RemoveIndex (Variables|StartingItems|GetNewStartingItems))
  (LootChest&StartingItems|StartDropping))

(fn GenerateUniqueID
  (params (ID :type Name))
  ;[1 1 1] Generates unique ID for item that is important for chest replication
  (return (Utilities|String|Append (Utilities|String|ToString(Name) ID) "_" (Utilities|String|ToString(Integer) (Math|Random|RandomIntegerinRange 10 9999)) (Utilities|Select :Index (Math|Random|RandomIntegerinRange 0 8) :Option%200 "A" :Option%201 "B" :Option%202 "C" :Option%203 "D" :Option%204 "E" :Option%205 "F" :Option%206 "H" :Option%207 "I" :Option%208 "J"))))

(fn SetUpItemFiltersArrayandSpecialSlotsCookingModule
  (bind _cookingmodule (Variables|Modules|GetCookingModule))
  (bind _cookingmodule_2 (Variables|Modules|GetCookingModule))
  (bind _cookingmodule_3 (Variables|Modules|GetCookingModule))
  (bind _cookingmodule_4 (Variables|Modules|GetCookingModule))
  (bind _cookingmodule_5 (Variables|Modules|GetCookingModule))
  (bind (_amountofcontentbars _amountofcontentslotsperbar) (Utilities|Struct|BreakS_ChestCookingModule _cookingmodule_3))
  (bind (_cookingslots_itemfilter _cookingslots_categoryfilter) (Utilities|Struct|BreakS_ChestCookingModule _cookingmodule_4))
  (bind (_contentslots_itemfilter _contentslots_categoryfilter) (Utilities|Struct|BreakS_ChestCookingModule _cookingmodule))
  (bind (_amountoffuelbars _amountoffuelslotsperbar) (Utilities|Struct|BreakS_ChestCookingModule _cookingmodule_5))
  (bind (_fuelslots_itemfilter _fuelslots_categoryfilter) (Utilities|Struct|BreakS_ChestCookingModule _cookingmodule_2))
  ;[1 1 1] only set up if cooking module is enabled
  (if (Utilities|Struct|BreakS_ChestCookingModule (Variables|Modules|GetCookingModule))
    ;[1 1 1] Set up filter arrays (note: order needs to fit slot order in UI)
    (for _index (range 1 (Utilities|Struct|BreakS_ChestCookingModule (Variables|Modules|GetCookingModule)))
      (Utilities|Array|Add (Variables|General|GetItemFilters) _cookingslots_itemfilter)
      (Utilities|Array|Add (Variables|General|GetCategoryFilters) _cookingslots_categoryfilter)
      (Utilities|Array|Add (Variables|General|GetSpecialSlots) "NewEnumerator1"))
    (for _index_2 (range 1 (* _amountoffuelbars _amountoffuelslotsperbar))
      (Utilities|Array|Add (Variables|General|GetItemFilters) _fuelslots_itemfilter)
      (Utilities|Array|Add (Variables|General|GetCategoryFilters) _fuelslots_categoryfilter)
      (Utilities|Array|Add (Variables|General|GetSpecialSlots) "NewEnumerator2"))
    (for _index_3 (range 1 (* _amountofcontentbars _amountofcontentslotsperbar))
      (Utilities|Array|Add (Variables|General|GetItemFilters) _contentslots_itemfilter)
      (Utilities|Array|Add (Variables|General|GetCategoryFilters) _contentslots_categoryfilter)
      (Utilities|Array|Add (Variables|General|GetSpecialSlots) "NewEnumerator0"))))

(fn SetUpInteractDuration
  ;[1 1 1] Set interact duration based on variable
  (bind _asbp_interaction_area (Utilities|Casting|CastToBP_InteractionArea (Variables|/Script/Engine.ChildActorComponent|GetChildActor (Variables|Default|GetInteractionTraceArea))))
  (Variables|/Game/AdvancedInventory/Blueprints/InteractionSystem/BP_InteractionArea.BP_InteractionArea_C|SetInteractDuration _asbp_interaction_area (Variables|SetUp|GetInteractDuration)))

(fn SetUpItemFiltersArrayandSpecialSlotsNormalChest
  (bind _chestmodule (Variables|Modules|GetChestModule))
  (bind (_itemfilter _categoryfilter) (Utilities|Struct|BreakS_ChestModule _chestmodule))
  (if (Utilities|Struct|BreakS_ChestModule (Variables|Modules|GetChestModule))
    (Utilities|Array|SetArrayElem (Variables|General|GetItemFilters) 0 _itemfilter true)
    (Utilities|Array|SetArrayElem (Variables|General|GetCategoryFilters) 0 _categoryfilter true)
    (Utilities|Array|SetArrayElem (Variables|General|GetSpecialSlots) 0 "NewEnumerator0" true)))