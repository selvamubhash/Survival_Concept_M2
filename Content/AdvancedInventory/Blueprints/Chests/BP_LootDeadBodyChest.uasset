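; Loot chest for a dead player's body that holds their inventory and equipment for about five minutes.
; LoadPlayerInventory unpacks serialized item strings into slot visibility and item arrays, placing equipment after the inventory slots.
; The server counts down on a one-second tick, then destroys both the character and the chest.
; The replicated countdown's OnRep refreshes the interact widget's timer and name only while it is visible.
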(event Custom|LoadPlayerInventory
  (params (CharacterComponentRef :type AC%20Inventory%20Character%20Component%20Object%20Reference) (AllItemsString :type String) (AllEquipSlots :type String))
  (bind _lootdeadplayermodule (Variables|Default|GetLootDeadPlayerModule))
  (bind (_inventoryamountofbars _inventoryamountofslotsperbar) (Utilities|Struct|BreakS_ChestLootDeadPlayerModule _lootdeadplayermodule))
  ;[1 1 1] Store player inventory in this chest (executed on server)
  (Variables|Default|SetCharacterComponentRef CharacterComponentRef)
  (bind _allslotsresult (CallFunction|LoadInventoryorEquipSlotsfromSingleString AllItemsString))
  (for (_array_element _array_index) _allslotsresult
    (Utilities|Array|SetArrayElem (Variables|Default|GetVisibility_AllSlots) _array_index (Utilities|Enum|NotEqual(Enum) _array_element ""))
    (if (Utilities|Enum|NotEqual(Enum) _array_element "")
      (Utilities|Array|SetArrayElem (Variables|Default|GetItemString_AllSlots) _array_index _array_element)))
  (bind _allslotsresult_2 (CallFunction|LoadInventoryorEquipSlotsfromSingleString AllEquipSlots))
  (for (_array_element_2 _array_index_2) _allslotsresult_2
    (if (Utilities|Enum|NotEqual(Enum) _array_element_2 "")
      (Utilities|Array|SetArrayElem (Variables|Default|GetVisibility_AllSlots) (+ _array_index_2 (* _inventoryamountofbars _inventoryamountofslotsperbar)) true)
      (Utilities|Array|SetArrayElem (Variables|Default|GetItemString_AllSlots) (+ _array_index_2 (* _inventoryamountofbars _inventoryamountofslotsperbar)) _array_element_2))))

(event EventBeginPlay
  ;[1 1 1] Start countdown on server
  (|CallParentFunction)
  (Networking|SwitchHasAuthority
    (:Authority
      (Variables|Default|SetCountdown (Math|Timespan|MakeTimespan 0 0 5 5))
      (Actor|Tick|SetActorTickEnabled true))))

(event EventTick
  (params (DeltaSeconds :type Float%20%28single-precision%29))
  ;[1 1 1] Tick is set to 1 second, decrease countdown by 1 second each time
  (Variables|Default|SetCountdown (- (Variables|Default|GetCountdown) (Math|Timespan|MakeTimespan 0 0 0 1)))
  ;;[1 1 1] If countdown reaches 0 seconds destroy character and this chest
  (if (Math|Boolean|ANDBoolean (<= (.Days (Math|Timespan|BreakTimespan (Media|MediaPlayer|GetDuration (Variables|Default|GetCountdown)))) 0) (<= (.Hours (Math|Timespan|BreakTimespan (Media|MediaPlayer|GetDuration (Variables|Default|GetCountdown)))) 0) (<= (.Minutes (Math|Timespan|BreakTimespan (Media|MediaPlayer|GetDuration (Variables|Default|GetCountdown)))) 0) (<= (.Seconds (Math|Timespan|BreakTimespan (Media|MediaPlayer|GetDuration (Variables|Default|GetCountdown)))) 0))
    (Actor|DestroyActor (Components|GetOwner (Variables|Default|GetCharacterComponentRef)))
    (Actor|DestroyActor)))

(fn ConstructionScript
  (|CallParentFunction))

(fn UpdateCountdownWidget
  ;[1 1 1] Update widget with new countdown data
  (bind _aswb_loot_dead_player_info (Utilities|Casting|CastToWB_LootDeadPlayerInfo (UserInterface|GetUserWidgetObject (Variables|Default|GetInteractWidget))))
  (Default|UpdateCountdown _aswb_loot_dead_player_info (Variables|Default|GetCountdown) (Variables|Default|GetName)))

(fn OnRepCountdown
  ;[1 1 1] Update widget for players who are currently tracing loot dead character
  (if (Rendering|IsVisible (Variables|Default|GetInteractWidget))
    (CallFunction|UpdateCountdownWidget)))