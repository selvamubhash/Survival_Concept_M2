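; BP_InteractionArea is an interaction area for a parent actor, relaying focus changes and access to that actor's interaction widget.
; On BeginPlay it caches the parent's "interact"-tagged widget component, then shows or hides it as focus toggles.
; Focus and widget requests special-case BP_0_Chest_Master, with interface messages for other parents.
; A customizable mesh defines its shape, hidden outside DEV mode.
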(event Custom|ToggleFocus
  (params (Focused :type Boolean))
  ;[1 1 1] toggle focus
  (Variables|Default|SetFocused Focused)
  (Development|SetHiddeninGame (Variables|Default|GetInteractWidgetComponentRef) (not (Variables|Default|GetFocused)) false)
  (bind _asbp_0_chest_master (Utilities|Casting|CastToBP_0_Chest_Master (Actor|GetParentActor))
    (:then
      (Default|ToggleFocus _asbp_0_chest_master (Variables|Default|GetFocused)))
    (:CastFailed
      (Class|BPInventoryInteractionInterface|ToggleFocusI(Message) (Actor|GetParentActor) (Variables|Default|GetFocused)))))

(event EventBeginPlay
  ;[1 1 1] set up
  (Variables|Default|SetInteractWidgetComponentRef (Utilities|Array|Get(acopy) (Actor|GetComponentsbyTag (Actor|GetParentActor) "/Script/UMG.WidgetComponent" "interact"))))

(fn ConstructionScript
  (Components|StaticMesh|SetStaticMesh (Variables|Default|GetShape) (Variables|Default|GetCustomShape))
  (if (not (Variables|Default|GetDEV))
    (Rendering|SetVisibility (Variables|Default|GetShape) false false)))

(fn GetInteractionWidget
  ;[1 1 1] get widget
  (if (== (Utilities|GetClass (Actor|GetParentActor)) "/Game/AdvancedInventory/Blueprints/Chests/BP_0_Chest_Master.BP_0_Chest_Master_C")
    (bind _asbp_0_chest_master (Utilities|Casting|CastToBP_0_Chest_Master (Actor|GetParentActor)))
    (return (Variables|/Game/AdvancedInventory/Blueprints/Chests/BP_0_Chest_Master.BP_0_Chest_Master_C|GetInteractWidget _asbp_0_chest_master))
    (else
      (bind _ref (Class|BPInventoryInteractionInterface|GetInteractionWidgetRefI(Message) (Actor|GetParentActor)))
      (return _ref))))