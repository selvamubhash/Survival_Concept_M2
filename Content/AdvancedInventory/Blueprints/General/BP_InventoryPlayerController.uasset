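; Player controller for the inventory system that routes player input to its ACInventoryPCComponent, which handles the actual logic.
; Input actions and keys drive hotbar selection, weapon aim, fire and reload, interaction, inspection, trading and inventory toggling.
; Possessing a pawn notifies the component of the respawn.
; Hardcoded development keys test durability, crafting unlocks, item grants and death, plus saving and loading player and server-side world data.
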(event EventPossess
  (params (PossessedPawn :type Pawn%20Object%20Reference))
  ;[1 1 1] OnPossess
  (Default|OnRespawnedonOwningClient (Variables|Default|GetAC_InventoryPC_Component) PossessedPawn))

(event Input|ActionEvents|InputActionInventoryAim
  (params (Key :type Key%20Structure))
  (bind _ac_inventorypc_component (Variables|Default|GetAC_InventoryPC_Component))
  ;[1 1 1] Weapon input
  (:Pressed
    (Default|Aim _ac_inventorypc_component true))
  (:Released
    (Default|Aim _ac_inventorypc_component false)))

(event Input|ActionEvents|InputActionInspect
  (params (Key :type Key%20Structure))
  (bind _ac_inventorypc_component (Variables|Default|GetAC_InventoryPC_Component))
  ;[1 1 1] General input
  (:Pressed
    (Default|Inspect _ac_inventorypc_component true))
  (:Released
    (Default|Inspect _ac_inventorypc_component false)))

(event Input|ActionEvents|InputActionConsumeItem
  (params (Key :type Key%20Structure))
  (bind _ac_inventorypc_component (Variables|Default|GetAC_InventoryPC_Component))
  ;[1 1 1] General input
  (:Pressed
    (Default|RightClickConsume _ac_inventorypc_component true))
  (:Released
    (Default|RightClickConsume _ac_inventorypc_component false)))

(event Input|ActionEvents|InputActionTradeInteractWihtPlayer
  (params (Key :type Key%20Structure))
  ;[1 1 1] General input
  (:Pressed
    (Default|InvitePlayertoTrade (Variables|Default|GetAC_InventoryPC_Component))))

(event Input|ActionEvents|InputActionTradeDecline
  (params (Key :type Key%20Structure))
  ;[1 1 1] General input
  (:Pressed
    (Default|DeclineTradeInvite (Variables|Default|GetAC_InventoryPC_Component))))

(event Input|ActionEvents|InputActionQuickEquipItem
  (params (Key :type Key%20Structure))
  ;[1 1 1] General input
  (:Pressed
    (Default|EquipArmorfromItem (Variables|Default|GetAC_InventoryPC_Component) true)))

(event Input|ActionEvents|InputActionFire
  (params (Key :type Key%20Structure))
  (bind _ac_inventorypc_component (Variables|Default|GetAC_InventoryPC_Component))
  ;[1 1 1] Weapon input
  (:Pressed
    (Default|TrytoShootwithWeapon _ac_inventorypc_component true))
  (:Released
    (Default|TrytoShootwithWeapon _ac_inventorypc_component false)))

(event Input|ActionEvents|InputActionToggleInventory
  (params (Key :type Key%20Structure))
  ;[1 1 1] General input
  (:Pressed
    (Default|ToggleInventoryVisibility (Variables|Default|GetAC_InventoryPC_Component))))

(event Input|ActionEvents|InputActionInteract
  (params (Key :type Key%20Structure))
  (bind _ac_inventorypc_component (Variables|Default|GetAC_InventoryPC_Component))
  ;[1 1 1] General input
  (:Pressed
    (Default|TrytoInteract _ac_inventorypc_component true))
  (:Released
    (Default|TrytoInteract _ac_inventorypc_component false)))

(event Input|ActionEvents|InputActionReloadWeapon
  (params (Key :type Key%20Structure))
  ;[1 1 1] Weapon input
  (:Pressed
    (Default|TrytoReloadCurrentWeapon (Variables|Default|GetAC_InventoryPC_Component))))

(event Input|KeyboardEvents|1
  (params (Key :type Key%20Structure))
  ;[1 1 1] Hotbar input
  (:Pressed
    (Default|SelectHotbarSlotKeyboard (Variables|Default|GetAC_InventoryPC_Component))))

(event Input|KeyboardEvents|O
  (params (Key :type Key%20Structure))
  ;[1 1 1] Devolopment inputs for testing
  ;;[1 1 1] Dev input to save player inventory
  (:Pressed
    (Utilities|IsValid (CallFunction|GetInventoryRef)
      (:Is%20Valid
        (Default|SaveOwnInventorySlots (Variables|Default|GetAC_InventoryPC_Component))
        (Default|SaveProfilePlayerData (Variables|Default|GetAC_InventoryPC_Component))
        (Default|SaveCraftingUnlockedStates (Variables|Default|GetAC_InventoryPC_Component))
        (Development|PrintString "Saved player data")))))

(event Input|KeyboardEvents|7
  (params (Key :type Key%20Structure))
  ;[1 1 1] Hotbar input
  (:Pressed
    (Default|SelectHotbarSlotKeyboard (Variables|Default|GetAC_InventoryPC_Component) 6)))

(event Input|KeyboardEvents|8
  (params (Key :type Key%20Structure))
  ;[1 1 1] Hotbar input
  (:Pressed
    (Default|SelectHotbarSlotKeyboard (Variables|Default|GetAC_InventoryPC_Component) 7)))

(event Input|KeyboardEvents|9
  (params (Key :type Key%20Structure))
  ;[1 1 1] Hotbar input
  (:Pressed
    (Default|SelectHotbarSlotKeyboard (Variables|Default|GetAC_InventoryPC_Component) 8)))

(event Input|MouseEvents|MouseWheelUp
  (params (Key :type Key%20Structure))
  ;[1 1 1] Hotbar input
  (:Pressed
    (Default|SelectHotbarSlotMouseWheel (Variables|Default|GetAC_InventoryPC_Component) true)))

(event Input|KeyboardEvents|L
  (params (Key :type Key%20Structure))
  ;[1 1 1] Devolopment inputs for testing
  ;;[1 1 1] Dev input to save player inventory
  (:Pressed
    (Utilities|IsValid (CallFunction|GetInventoryRef)
      (:Is%20Valid
        (Default|LoadOwnInventorySlots (Variables|Default|GetAC_InventoryPC_Component))
        (Default|LoadProfilePlayerData (Variables|Default|GetAC_InventoryPC_Component))
        (Default|LoadCraftingUnlockedStates (Variables|Default|GetAC_InventoryPC_Component))
        (Development|PrintString "Loaded player data")))))

(event Input|KeyboardEvents|M
  (params (Key :type Key%20Structure))
  (bind _inventory (CallFunction|GetInventoryRef))
  ;[1 1 1] Devolopment inputs for testing
  (:Pressed
    (Utilities|IsValid _inventory
      (:Is%20Valid
        (Default|UnlockCraftableItem (Variables|/Game/AdvancedInventory/Widgets/InventoryGeneral/WB_Inventory.WB_Inventory_C|GetRef_CraftingMenu _inventory) "ironboots" true true)))))

(event Input|KeyboardEvents|CtrlO
  (params (Key :type Key%20Structure))
  ;[1 1 1] Devolopment inputs for testing
  ;;[1 1 1] Dev input to save chest, ground items & vendors (trigger these events on server)
  (:Pressed
    (Utilities|IsValid (CallFunction|GetInventoryRef)
      (:Is%20Valid
        (Default|SaveChestSlots (Variables|Default|GetAC_InventoryPC_Component) true) ; Should only be executed on server
        (Default|SaveGroundItems (Variables|Default|GetAC_InventoryPC_Component) true) ; Should only be executed on server
        (Default|SaveVendors (Variables|Default|GetAC_InventoryPC_Component) true) ; Should only be executed on server
        (Development|PrintString "Saved server data")))))

(event Input|KeyboardEvents|Z
  (params (Key :type Key%20Structure))
  ;[1 1 1] Devolopment inputs for testing
  (:Pressed
    (Utilities|IsValid (CallFunction|GetInventoryRef)
      (:Is%20Valid
        (Default|AdjustDurabilityOfCurrentHotbarItemonClient (Variables|Default|GetAC_InventoryPC_Component) "NewEnumerator0" 0.0)))))

(event Input|KeyboardEvents|N
  (params (Key :type Key%20Structure))
  (bind _inventory (CallFunction|GetInventoryRef))
  ;[1 1 1] Devolopment inputs for testing
  (:Pressed
    (Utilities|IsValid _inventory
      (:Is%20Valid
        (Default|UnlockCraftableItem (Variables|/Game/AdvancedInventory/Widgets/InventoryGeneral/WB_Inventory.WB_Inventory_C|GetRef_CraftingMenu _inventory) "legharness" true true)))))

(event Input|KeyboardEvents|CtrlL
  (params (Key :type Key%20Structure))
  ;[1 1 1] Devolopment inputs for testing
  ;;[1 1 1] Dev input to save chest, ground items & vendors (trigger these events on server)
  (:Pressed
    (Utilities|IsValid (CallFunction|GetInventoryRef)
      (:Is%20Valid
        (Default|LoadChestSlots (Variables|Default|GetAC_InventoryPC_Component) true) ; Should only be executed on server
        (Default|LoadGroundItems (Variables|Default|GetAC_InventoryPC_Component) true) ; Should only be executed on server
        (Default|LoadVendors (Variables|Default|GetAC_InventoryPC_Component) true) ; Should only be executed on server
        (Development|PrintString "Loaded server data")))))

(event Input|KeyboardEvents|B
  (params (Key :type Key%20Structure))
  (bind _inventory (CallFunction|GetInventoryRef))
  ;[1 1 1] Devolopment inputs for testing
  (:Pressed
    (Utilities|IsValid _inventory
      (:Is%20Valid
        (Default|UnlockCraftableItem (Variables|/Game/AdvancedInventory/Widgets/InventoryGeneral/WB_Inventory.WB_Inventory_C|GetRef_CraftingMenu _inventory) "chestharness" true true)))))

(event Input|KeyboardEvents|G
  (params (Key :type Key%20Structure))
  ;[1 1 1] Devolopment inputs for testing
  (:Pressed
    (Utilities|IsValid (CallFunction|GetInventoryRef)
      (:Is%20Valid
        (bind _outrownames (DataTable|GetDataTableRowNames "/Game/AdvancedInventory/ItemDataTables/CategorizedItemTables/DT_Resources.DT_Resources"))
        (for _array_element _outrownames
          (Default|AddItemSimple (CallFunction|GetInventoryRef) _array_element 10))))))

(event Input|MouseEvents|MouseWheelDown
  (params (Key :type Key%20Structure))
  ;[1 1 1] Hotbar input
  (:Pressed
    (Default|SelectHotbarSlotMouseWheel (Variables|Default|GetAC_InventoryPC_Component) false)))

(event Input|KeyboardEvents|CtrlX
  (params (Key :type Key%20Structure))
  ;[1 1 1] Devolopment inputs for testing
  (:Pressed
    (Utilities|IsValid (CallFunction|GetInventoryRef)
      (:Is%20Valid
        (Default|EventonPlayerDeath (Variables|Default|GetAC_InventoryPC_Component))))))

(event Input|KeyboardEvents|2
  (params (Key :type Key%20Structure))
  ;[1 1 1] Hotbar input
  (:Pressed
    (Default|SelectHotbarSlotKeyboard (Variables|Default|GetAC_InventoryPC_Component) 1)))

(event Input|KeyboardEvents|3
  (params (Key :type Key%20Structure))
  ;[1 1 1] Hotbar input
  (:Pressed
    (Default|SelectHotbarSlotKeyboard (Variables|Default|GetAC_InventoryPC_Component) 2)))

(event Input|KeyboardEvents|4
  (params (Key :type Key%20Structure))
  ;[1 1 1] Hotbar input
  (:Pressed
    (Default|SelectHotbarSlotKeyboard (Variables|Default|GetAC_InventoryPC_Component) 3)))

(event Input|KeyboardEvents|5
  (params (Key :type Key%20Structure))
  ;[1 1 1] Hotbar input
  (:Pressed
    (Default|SelectHotbarSlotKeyboard (Variables|Default|GetAC_InventoryPC_Component) 4)))

(event Input|KeyboardEvents|6
  (params (Key :type Key%20Structure))
  ;[1 1 1] Hotbar input
  (:Pressed
    (Default|SelectHotbarSlotKeyboard (Variables|Default|GetAC_InventoryPC_Component) 5)))

(fn ConstructionScript)