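; World pickup actor for a dropped or map-placed inventory item, showing a static mesh, skeletal mesh or child actor from item data.
; Replicated item data triggers setup for player drops, which are tossed with projectile movement and can expire via a lifetime component.
; Nearby items with matching IDs merge amounts, while overlap boxes and line traces free items from blocking objects or let them fall.
; Hover and spin animations pause when not rendered.
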(event OnProjectileStop(ProjectileMovement)
  (params (ImpactResult :type Hit%20Result%20Structure%20%28by%20ref%29))
  ;[1 1 1] If another item with the same ID comes in the radius of this item, the items will be merged
  (Utilities|FlowControl|Sequence
    (:then_0
      (if (> (Utilities|Array|Length (Collision|GetOverlappingActors (Variables|Default|GetBoxAvoidGettingStuckWithOtherItems) "BP_DropItemActor_C" :!class /Script/Engine.PrimitiveComponent)) 2)
        (CallFunction|ReactivateProjectileMovement true)))
    (:then_1
      (Utilities|FlowControl|Delay 0.4)
      (bind _array_element (Utilities|Array|ForEachLoopwithBreak (Collision|GetOverlappingActors "BP_DropItemActor_C" :!class /Script/Engine.Actor) :!label _label)
        (:LoopBody
          (if (!= _array_element self)
            (bind _asbp_drop_item_actor (Utilities|Casting|CastToBP_DropItemActor _array_element))
            (if (and (or (Utilities|Struct|BreakS_AdditionalGeneralData (.AdditionalGeneralData (Utilities|Struct|BreakS_ItemData (Variables|General|GetItemDataNew)))) (Variables|General|GetbMergeAlsoNotStackableItems)) (Utilities|Name|Equal(Name) (.ID (Utilities|Struct|BreakS_ItemData (Variables|BP_DropItemActor_C|GetItemDataNew _asbp_drop_item_actor))) (.ID (Utilities|Struct|BreakS_ItemData (Variables|General|GetItemDataNew)))))
              (CallFunction|IncreaseAmountAnimation _asbp_drop_item_actor)
              (bind _structout (Utilities|Struct|SetmembersinS_ItemData (Variables|General|GetItemDataNew) (+ (.Amount (Utilities|Struct|BreakS_ItemData (Variables|BP_DropItemActor_C|GetItemDataNew _asbp_drop_item_actor))) (.Amount (Utilities|Struct|BreakS_ItemData (Variables|General|GetItemDataNew))))))
              (Variables|BP_DropItemActor_C|SetItemDataNew _asbp_drop_item_actor _structout)
              (Actor|DestroyActor)
              (goto _label Break))))))))

(event OnComponentBeginOverlap(BoxTop)
  (params (OverlappedComponent :type Primitive%20Component%20Object%20Reference) (OtherActor :type Actor%20Object%20Reference) (OtherComp :type Primitive%20Component%20Object%20Reference) (OtherBodyIndex :type Integer) (bFromSweep :type Boolean) (SweepResult :type Hit%20Result%20Structure%20%28by%20ref%29))
  ;[1 1 1] If item collides with a PlacingObject, a new location is necessary
  (if (Variables|General|GetbFindWayOutIfBlockedByDefinedObject)
    (bind (_location _itemshouldfalldown_) (CallFunction|FindWayOut))
    (Transformation|SetActorLocation (Math|Vector|MakeVector (.X (Math|Vector|BreakVector _location)) (.Y (Math|Vector|BreakVector _location)) (+ (.Z (Math|Vector|BreakVector _location)) 3e+01)) false false)
    (if _itemshouldfalldown_
      (CallFunction|ReactivateProjectileMovement false))))

(event OnComponentEndOverlap(BoxDown)
  (params (OverlappedComponent :type Primitive%20Component%20Object%20Reference) (OtherActor :type Actor%20Object%20Reference) (OtherComp :type Primitive%20Component%20Object%20Reference) (OtherBodyIndex :type Integer))
  ;[1 1 1] If item is on the top of a PlacingObject and this object gets destroyed ist is necessary that the item falls down
  (if (Variables|General|GetbFindWayOutIfBlockedByDefinedObject)
    (CallFunction|ReactivateProjectileMovement false)))

(event OnProjectileStop(NewProjectileMovement)
  (params (ImpactResult :type Hit%20Result%20Structure%20%28by%20ref%29))
  ;[1 1 1] If another item with the same ID comes in the radius of this item, the items will be merged
  (Utilities|FlowControl|Sequence
    (:then_0
      (if (> (Utilities|Array|Length (Collision|GetOverlappingActors (Variables|Default|GetBoxAvoidGettingStuckWithOtherItems) "BP_DropItemActor_C" :!class /Script/Engine.PrimitiveComponent)) 2)
        (CallFunction|ReactivateProjectileMovement true)))
    (:then_1
      (Utilities|FlowControl|Delay 0.4)
      (bind _array_element (Utilities|Array|ForEachLoopwithBreak (Collision|GetOverlappingActors "BP_DropItemActor_C" :!class /Script/Engine.Actor) :!label _label)
        (:LoopBody
          (if (!= _array_element self)
            (bind _asbp_drop_item_actor (Utilities|Casting|CastToBP_DropItemActor _array_element))
            (if (and (or (Utilities|Struct|BreakS_AdditionalGeneralData (.AdditionalGeneralData (Utilities|Struct|BreakS_ItemData (Variables|General|GetItemDataNew)))) (Variables|General|GetbMergeAlsoNotStackableItems)) (Utilities|Name|Equal(Name) (.ID (Utilities|Struct|BreakS_ItemData (Variables|BP_DropItemActor_C|GetItemDataNew _asbp_drop_item_actor))) (.ID (Utilities|Struct|BreakS_ItemData (Variables|General|GetItemDataNew)))))
              (CallFunction|IncreaseAmountAnimation _asbp_drop_item_actor)
              (bind _structout (Utilities|Struct|SetmembersinS_ItemData (Variables|General|GetItemDataNew) (+ (.Amount (Utilities|Struct|BreakS_ItemData (Variables|BP_DropItemActor_C|GetItemDataNew _asbp_drop_item_actor))) (.Amount (Utilities|Struct|BreakS_ItemData (Variables|General|GetItemDataNew))))))
              (Variables|BP_DropItemActor_C|SetItemDataNew _asbp_drop_item_actor _structout)
              (Actor|DestroyActor)
              (goto _label Break))))))))

(event OnComponentBeginOverlap(RadiusForItemMerging)
  (params (OverlappedComponent :type Primitive%20Component%20Object%20Reference) (OtherActor :type Actor%20Object%20Reference) (OtherComp :type Primitive%20Component%20Object%20Reference) (OtherBodyIndex :type Integer) (bFromSweep :type Boolean) (SweepResult :type Hit%20Result%20Structure%20%28by%20ref%29))
  ;[1 1 1] If another item with the same ID comes in the radius of this item, the items will be merged
  (bind _array_element (Utilities|Array|ForEachLoopwithBreak (Collision|GetOverlappingActors "BP_DropItemActor_C" :!class /Script/Engine.Actor) :!label _label)
    (:LoopBody
      (if (!= _array_element self)
        (bind _asbp_drop_item_actor (Utilities|Casting|CastToBP_DropItemActor _array_element))
        (if (and (or (Utilities|Struct|BreakS_AdditionalGeneralData (.AdditionalGeneralData (Utilities|Struct|BreakS_ItemData (Variables|General|GetItemDataNew)))) (Variables|General|GetbMergeAlsoNotStackableItems)) (Utilities|Name|Equal(Name) (.ID (Utilities|Struct|BreakS_ItemData (Variables|BP_DropItemActor_C|GetItemDataNew _asbp_drop_item_actor))) (.ID (Utilities|Struct|BreakS_ItemData (Variables|General|GetItemDataNew)))))
          (CallFunction|IncreaseAmountAnimation _asbp_drop_item_actor)
          (bind _structout (Utilities|Struct|SetmembersinS_ItemData (Variables|General|GetItemDataNew) (+ (.Amount (Utilities|Struct|BreakS_ItemData (Variables|BP_DropItemActor_C|GetItemDataNew _asbp_drop_item_actor))) (.Amount (Utilities|Struct|BreakS_ItemData (Variables|General|GetItemDataNew))))))
          (Variables|BP_DropItemActor_C|SetItemDataNew _asbp_drop_item_actor _structout)
          (Actor|DestroyActor)
          (goto _label Break))))))

(event Custom|ShowNewInfoWidget
  (params (Show? :type Boolean))
  ;[1 1 1] Show new info pick up widget
  (Development|SetHiddeninGame (Variables|Default|GetWidget) (not Show?) false)
  (bind _aswb_new_info_pick_up (Utilities|Casting|CastToWB_NewInfoPickUp (UserInterface|GetUserWidgetObject (Variables|Default|GetWidget))))
  (Default|UpdatePickUpInfo _aswb_new_info_pick_up (Variables|General|GetItemDataNew)))

(event Custom|ActivateItemMergeAfterDealay
  ;[1 1 1] Delayed make it possible to merge
  (Networking|SwitchHasAuthority
    (:Authority
      (Utilities|FlowControl|Delay 0.4)
      (Collision|SetCollisionEnabled (Variables|Default|GetRadiusForItemMerging) "QueryOnly"))))

(event Custom|IncreaseAmountAnimation
  ;[1 1 1] Animation of the scale when the amount gets increased
  (if (Variables|Other|GetbRendered)
    (if (not (Audio|Components|Audio|IsPlaying (Variables|Default|GetAddingAnimation)))
      (bind _newtrack_0 (Timeline|AddingAnimation PlayFromStart)
        (:Update
          (Transformation|SetRelativeScale3D (Variables|Default|GetRotationAnimation_Scene) (Math|Conversions|ToVector(Float) (Math|Float|Lerp 1.0 1.2 _newtrack_0))))))))

(event Custom|EnableGroundListOverlap
  ;[1 1 1] Delayed make it possible to get recognized by ground list detection
  (Utilities|FlowControl|Delay 0.41)
  (Collision|SetCollisionEnabled (Variables|Default|GetGroundListOverlap) "NoCollision")
  (Collision|SetCollisionEnabled (Variables|Default|GetGroundListOverlap) "QueryOnly"))

(event Custom|ShowActorWhenItsFullyLoaded
  ;[1 1 1] Server validation to show actor at beginning
  (Rendering|SetActorHiddenInGame false))

(event Custom|StartHover
  ;[1 1 1] Hover and rotation animation
  (if (Variables|General|GetbEnableHover)
    (Utilities|FlowControl|Sequence
      (:then_0
        (Components|MoveComponentTo (Variables|Default|GetSpringArm) (Math|Vector|MakeVector 0.0 0.0 (Math|Random|RandomFloatinRange 2.0 3.5)) "0, 0, 0" true true 2.0 true :!label _label)
        (if (Variables|Other|GetbRendered)
          (Components|MoveComponentTo (Variables|Default|GetSpringArm) (Math|Vector|MakeVector 0.0 0.0 (Math|Random|RandomFloatinRange -2.0 -3.5)) "0, 0, 0" true true 2.0 true)
          (if (Variables|Other|GetbRendered)
            (goto _label))))
      (:then_1
        (Components|MoveComponentTo (Variables|Default|GetRotationAnimation_Scene) "0, 0, 0" (Math|Rotator|MakeRotator 0.0 0.0 (+ (.Yaw (Math|Rotator|BreakRotator (Variables|/Script/Engine.SceneComponent|GetRelativeRotation (Variables|Default|GetRotationAnimation_Scene)))) 16.0)) false false 2.0 true :!label _label_2)
        (if (Variables|Other|GetbRendered)
          (goto _label_2))))))

(event Custom|ForceStopHover
  ;[1 1 1] Hover and rotation animation
  (Utilities|FlowControl|Sequence
    (:then_0
      (Components|MoveComponentTo (Variables|Default|GetSpringArm) (Math|Vector|MakeVector 0.0 0.0 (Math|Random|RandomFloatinRange 2.0 3.5)) "0, 0, 0" true true 2.0 true) ; enters at Stop
    )
    (:then_1
      (Components|MoveComponentTo (Variables|Default|GetSpringArm) (Math|Vector|MakeVector 0.0 0.0 (Math|Random|RandomFloatinRange -2.0 -3.5)) "0, 0, 0" true true 2.0 true) ; enters at Stop
    )
    (:then_2
      (Components|MoveComponentTo (Variables|Default|GetRotationAnimation_Scene) "0, 0, 0" (Math|Rotator|MakeRotator 0.0 0.0 (+ (.Yaw (Math|Rotator|BreakRotator (Variables|/Script/Engine.SceneComponent|GetRelativeRotation (Variables|Default|GetRotationAnimation_Scene)))) 16.0)) false false 2.0 true) ; enters at Stop
    )))

(event Custom|Update
  (params (ItemData :type S%20Item%20Data%20Structure))
  ;[1 1 1] Update Item Data (will be executed on server only)
  (Variables|General|SetItemDataNew ItemData))

(event EventBeginPlay
  ;[1 1 1] Event Begin Play & Set up
  (CallFunction|StartHover)
  (Utilities|FlowControl|Sequence
    (:then_0
      (if (Utilities|Struct|BreakS_SpawnItemSettings (Variables|General|GetStartingItemData))
        (Variables|Other|SetbAlreadySpawned true)
        (Utilities|FlowControl|Sequence
          (:then_0
            (SetUp|SetUpatStart))
          (:then_1
            (Networking|SwitchHasAuthority
              (:Authority
                (CallFunction|ShowActorwhenItsFullyLoaded)))))))
    (:then_1
      (Networking|SwitchHasAuthority
        (:Authority
          (if (> (Variables|General|GetLifetimeInMinutes) 0)
            (bind _returnvalue (AddComponent|AddACItemActorLifetime))
            (Default|Start _returnvalue (Variables|General|GetLifetimeInMinutes))))))))

(event EventTick
  (params (DeltaSeconds :type Float%20%28single-precision%29))
  (bind _returnvalue (Class|Actor|WasRecentlyRendered 0.1))
  ;[1 1 1] Event Tick to save performane by stopping hover and other effects if it is not rendered
  (if (Math|Boolean|NotEqual(Boolean) _returnvalue (Variables|Other|GetbRendered))
    (bind _output_get (Variables|Other|SetbRendered _returnvalue))
    (if _output_get
      (CallFunction|StartHover)
      (else
        (CallFunction|ForceStopHover)))))

(fn ConstructionScript
  (bind _startingitemdata (Variables|General|GetStartingItemData))
  (bind (_busestartingitemdata _startingitemdata_2) (Utilities|Struct|BreakS_SpawnItemSettings _startingitemdata))
  ;[1 1 1] Show item in editor
  (if (Variables|General|GetSpawnAtStart)
    (if _busestartingitemdata
      (bind (_out_row _found) (CallFunction|GetItemDatabyID (Utilities|Struct|BreakDataTableRowHandle _startingitemdata_2)))
      (if _found
        (switch Utilities|FlowControl|Switch|SwitchonE_ItemActorMeshType (Utilities|Struct|BreakS_AdditionalGeneralData (Utilities|Struct|BreakS_ItemData _out_row))
          (:NewEnumerator0
            (Components|StaticMesh|SetStaticMesh (Variables|Default|GetItemStaticMesh) (.StaticMesh (Utilities|Struct|BreakS_AdditionalGeneralData (Utilities|Struct|BreakS_ItemData _out_row))))
            (Transformation|SetRelativeTransform (Variables|Default|GetItemStaticMesh) (.DropItemTransform (Utilities|Struct|BreakS_AdditionalGeneralData (Utilities|Struct|BreakS_ItemData _out_row))) false false)
            (Rendering|SetVisibility (Variables|Default|GetItemSkeletalMesh) false false))
          (:NewEnumerator1
            (Components|SkinnedMesh|SetSkinnedAssetandUpdate (Variables|Default|GetItemSkeletalMesh) (.SkeletalMesh (Utilities|Struct|BreakS_AdditionalGeneralData (Utilities|Struct|BreakS_ItemData _out_row))) true)
            (Transformation|SetRelativeTransform (Variables|Default|GetItemSkeletalMesh) (.DropItemTransform (Utilities|Struct|BreakS_AdditionalGeneralData (Utilities|Struct|BreakS_ItemData _out_row))) false false)
            (Rendering|SetVisibility (Variables|Default|GetItemStaticMesh) false false))
          (:NewEnumerator2
            (ChildActorComponent|SetChildActorClass (Variables|Default|GetItemChildActor) (.Actor (Utilities|Struct|BreakS_AdditionalGeneralData (Utilities|Struct|BreakS_ItemData _out_row))))
            (Transformation|SetRelativeTransform (Variables|Default|GetItemStaticMesh) (.DropItemTransform (Utilities|Struct|BreakS_AdditionalGeneralData (Utilities|Struct|BreakS_ItemData _out_row))) false false)
            (Rendering|SetVisibility (Variables|Default|GetItemStaticMesh) false false)))))))

(fn ReactivateProjectileMovement
  (params (drop? :type Boolean))
  (bind _projectilemovement (Variables|Default|GetProjectileMovement))
  ;[1 1 1] Destroy the current ProjectileComponent and create a new one
  (Utilities|IsValid _projectilemovement
    (:Is%20Valid
      (Components|DestroyComponent _projectilemovement))
    (:Is%20Not%20Valid
      (Utilities|IsValid (Variables|Default|GetNewProjectileMovement)
        (:Is%20Valid
          (Components|DestroyComponent (Variables|Default|GetNewProjectileMovement)))
        (:Is%20Not%20Valid
          _))))
  (bind _returnvalue (AddComponent|AddProjectileMovementComponent))
  (bind _output_get (Variables|Default|SetNewProjectileMovement _returnvalue))
  (if drop?
    (Game|Components|ProjectileMovement|SetVelocityinLocalSpace _output_get (Math|Vector|MakeVector 1.5e+02 1.5e+02 3.5e+02))
    (Variables|/Script/Engine.ProjectileMovementComponent|SetbShouldBounce _output_get true)
    (Variables|/Script/Engine.ProjectileMovementComponent|SetFriction _output_get 0.2)
    (Variables|/Script/Engine.ProjectileMovementComponent|SetBounciness _output_get 0.2)))

(fn FindWayOut
  ;[1 1 1] The function checks all directions (not bottom). Distance of Linetrace 0: Linetrace is still in a Object of the type "PlacingObject"   I   Distance of the Linetrace >0: Linetrace does not collide with a PlacingObject -> ReturnsLocation
  (Math|Integer|IncrementInt (LocalVariables|Getcount2) :!label _label
    (:%20%20
      (for _index (range 0 4)
        (bind _output_get (LocalVariables|SetcheckDirection (Utilities|Select :Index _index :Option%200 "0, 0,50.000000" :Option%201 "0,-50.000000, 0" :Option%202 "0,50.000000, 0" :Option%203 "50.000000, 0, 0" :Option%204 "-50.000000, 0, 0")))
        (bind _outhit (Collision|LineTraceByChannel (+ (* _output_get (+ (LocalVariables|Getcount2) 1)) (Transformation|GetActorLocation) "0,0.000000,15.000000") (+ (* _output_get (LocalVariables|Getcount2)) (Transformation|GetActorLocation) "0,0.000000,15.000000") "TraceTypeQuery3" false 0 "None"))
        (if (not (== (.Distance (Collision|BreakHitResult _outhit)) 0.0))
          (return (+ (.Location (Collision|BreakHitResult _outhit)) (select (== _index 0) "0, 0, 0" (LocalVariables|GetcheckDirection))) (not (== _index 0)))))
      (goto _label))))

(fn SetUpatStart
  ;[1 1 1] Set up at start - applies if placed in map and not spawned during game
  (bind (_out_row _found) (CallFunction|GetItemDatabyID (Utilities|Struct|BreakDataTableRowHandle (.StartingItemData (Utilities|Struct|BreakS_SpawnItemSettings (Variables|General|GetStartingItemData))))))
  (if _found
    (Variables|General|SetItemDataNew _out_row)
    (Utilities|Struct|SetmembersinS_ItemData (Variables|General|GetItemDataNew) (Variables|General|GetAmount_AtStart))
    (Components|Movement|SetUpdatedComponent (Variables|Default|GetProjectileMovement) (Variables|Default|GetitemCollisionMesh))
    (SetUp|SetMeshorActor)
    (CallFunction|ActivateItemMergeAfterDealay)))

(fn SetUpNotatStart
  (bind _projectilemovement (Variables|Default|GetProjectileMovement))
  ;[1 1 1] Set up after spawn during game (dropped from player)
  (Variables|Other|SetbAlreadySpawned true)
  (Utilities|IsValid _projectilemovement
    (:Is%20Valid
      (Game|Components|ProjectileMovement|SetVelocityinLocalSpace _projectilemovement (Math|Vector|MakeVector 3.5e+02 0.0 (Variables|Other|GetzVelocity)))
      (Components|Movement|SetUpdatedComponent (Variables|Default|GetProjectileMovement) (Variables|Default|GetitemCollisionMesh))
      (Rendering|SetActorHiddenInGame false)
      (SetUp|SetMeshorActor)
      (CallFunction|ActivateItemMergeAfterDealay))))

(fn SetMeshorActor
  (bind _itemdatanew (Variables|General|GetItemDataNew))
  (bind _additionalgeneraldata (Utilities|Struct|BreakS_ItemData _itemdatanew))
  (bind (_skeletalmesh _dropitemtransform) (Utilities|Struct|BreakS_AdditionalGeneralData _additionalgeneraldata))
  (bind (_actor _dropitemtransform_2) (Utilities|Struct|BreakS_AdditionalGeneralData _additionalgeneraldata))
  (bind (_staticmesh _dropitemtransform_3) (Utilities|Struct|BreakS_AdditionalGeneralData _additionalgeneraldata))
  ;[1 1 1] Set up skeletal/static mesh or child actor class based on item data
  (switch Utilities|FlowControl|Switch|SwitchonE_ItemActorMeshType (Utilities|Struct|BreakS_AdditionalGeneralData _additionalgeneraldata)
    (:NewEnumerator0
      (Components|StaticMesh|SetStaticMesh (Variables|Default|GetItemStaticMesh) _staticmesh)
      (Transformation|SetRelativeTransform (Variables|Default|GetItemStaticMesh) _dropitemtransform_3 false false))
    (:NewEnumerator1
      (Components|SkinnedMesh|SetSkinnedAssetandUpdate (Variables|Default|GetItemSkeletalMesh) _skeletalmesh true)
      (Transformation|SetRelativeTransform (Variables|Default|GetItemSkeletalMesh) _dropitemtransform false false))
    (:NewEnumerator2
      (ChildActorComponent|SetChildActorClass (Variables|Default|GetItemChildActor) _actor)
      (Transformation|SetRelativeTransform (Variables|Default|GetItemChildActor) _dropitemtransform_2 false false))))

(fn OnRepItemDataNew
  ;[1 1 1] Executed for everyone if item data updated
  (CallFunction|EnableGroundlistOverlap)
  (if (.bUseStartingItemData (Utilities|Struct|BreakS_SpawnItemSettings (Variables|General|GetStartingItemData)))
    _
    (else
      (SetUp|SetUpNotatStart)))
  (if (Rendering|IsVisible (Variables|Default|GetWidget))
    (bind _aswb_new_info_pick_up (Utilities|Casting|CastToWB_NewInfoPickUp (UserInterface|GetUserWidgetObject (Variables|Default|GetWidget))))
    (Default|UpdatePickUpInfo _aswb_new_info_pick_up (Variables|General|GetItemDataNew))))