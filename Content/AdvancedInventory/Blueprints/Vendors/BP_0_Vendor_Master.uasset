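; Base vendor Blueprint for the inventory system, holding a product list seeded with randomized AI stock.
; On BeginPlay, the authority rolls each starting product's offer chance, looks up vendor-enabled item data, and randomizes amount, quantity and durability.
; Each product gets a multiplier-scaled price, an item-based description and a random-suffixed ID, then AddProduct appends it to Products.
; An interface event forwards focus changes to CallOnFocus.
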(event Custom|AddProduct
  (params (product%20data :type S%20Vendor%20Product%20Structure))
  ;[1 1 1] Add product to products array on server
  (Utilities|Array|Add (Variables|Default|GetProducts) product%20data))

(event EventBeginPlay
  ;[1 1 1] Set up starting products
  (Networking|SwitchHasAuthority
    (:Authority
      (for _array_element (Variables|Default|GetAI_StartingProducts)
        (bind (_add_ _productdata) (CallFunction|CreateAIStartingProduct _array_element))
        (if _add_
          (CallFunction|AddProduct _productdata))))))

(event EventToggleFocusI
  (params (Focus :type Boolean))
  ;[1 1 1] Focusing vendor
  (Default|CallOnFocus Focus))

(fn ConstructionScript)

(fn CreateAIStartingProduct
  (params (Product :type S%20AI%20Vendor%20Product%20Structure))
  (LocalVariables|SetAI_StartingProduct_Local Product)
  ;[1 1 1] Generate random number and continue based on probability
  (bind _output_get (LocalVariables|SetRandomProbability_Local (Math|Random|RandomIntegerinRange 0 100)))
  (if (>= (Utilities|Struct|BreakS_AI_VendorProduct (LocalVariables|GetAI_StartingProduct_Local)) _output_get)
    ;[1 1 1] Save item data based on ID in variable
    (bind (_out_row _found) (CallFunction|GetItemDatabyID (Utilities|Struct|BreakDataTableRowHandle (Utilities|Struct|BreakS_AI_VendorProduct (LocalVariables|GetAI_StartingProduct_Local)))))
    (if _found
      (LocalVariables|SetCurrentItemData_Local _out_row)
      ;[1 1 1] check if vendor module is enabled for this item
      (if (Utilities|Struct|BreakS_Vendor (Utilities|Struct|BreakS_ItemData (LocalVariables|GetCurrentItemData_Local)))
        ;[1 1 1] set amount
        (if (not (Utilities|Struct|BreakS_AdditionalGeneralData (Utilities|Struct|BreakS_ItemData (LocalVariables|GetCurrentItemData_Local))))
          (LocalVariables|SetAmount_Local 1)
          (else
            (LocalVariables|SetAmount_Local (Math|Random|RandomIntegerinRange (.AmountMin (Utilities|Struct|BreakS_AI_VendorProduct (LocalVariables|GetAI_StartingProduct_Local))) (.AmountMax (Utilities|Struct|BreakS_AI_VendorProduct (LocalVariables|GetAI_StartingProduct_Local)))))))
        ;[1 1 1] Prevent adding if amount is 0 or less
        (if (> (LocalVariables|GetAmount_Local) 0)
          ;[1 1 1] Update amount in item data
          (Utilities|Struct|SetmembersinS_ItemData (LocalVariables|GetCurrentItemData_Local) (LocalVariables|GetAmount_Local))
          ;[1 1 1] Set random quantitiy
          (LocalVariables|SetQuantity_Local (Math|Random|RandomIntegerinRange (.QuantityMin (Utilities|Struct|BreakS_AI_VendorProduct (LocalVariables|GetAI_StartingProduct_Local))) (.QuantityMax (Utilities|Struct|BreakS_AI_VendorProduct (LocalVariables|GetAI_StartingProduct_Local)))))
          ;[1 1 1] Set random durability if item has durability
          (if (.Enabled (Utilities|Struct|BreakS_Durability (Utilities|Struct|BreakS_ItemData (LocalVariables|GetCurrentItemData_Local))))
            (Utilities|Struct|SetmembersinS_Durability (Utilities|Struct|BreakS_ItemData (LocalVariables|GetCurrentItemData_Local)) (Math|Float|Lerp 0.0 (.MaxDurability (Utilities|Struct|BreakS_Durability (Utilities|Struct|BreakS_ItemData (LocalVariables|GetCurrentItemData_Local)))) (/ (Math|Conversions|ToFloat(Integer) (Math|Random|RandomIntegerinRange (.DurabilityPercentMin_0_to_100 (Utilities|Struct|BreakS_AI_VendorProduct (LocalVariables|GetAI_StartingProduct_Local))) (.DurabilityPercentMax_0_to_100 (Utilities|Struct|BreakS_AI_VendorProduct (LocalVariables|GetAI_StartingProduct_Local))))) 1e+02))))
          ;[1 1 1] Return whole product data
          (return true (Utilities|Struct|MakeS_VendorProduct (LocalVariables|GetCurrentItemData_Local) (Math|Float|Truncate (* (LocalVariables|GetAmount_Local) (* (Utilities|Struct|BreakS_Vendor (.Vendor (Utilities|Struct|BreakS_ItemData (LocalVariables|GetCurrentItemData_Local)))) (Variables|Default|GetAI_PriceMultiplier)))) (LocalVariables|GetQuantity_Local) (LocalVariables|GetAmount_Local) (CallFunction|AIDescriptionbyID (.ID (Utilities|Struct|BreakS_ItemData (LocalVariables|GetCurrentItemData_Local)))) 0 "" "ShopOwner" (CallFunction|GeneratePrdouctID (CallFunction|ItemDatatoString (LocalVariables|GetCurrentItemData_Local)))))
          (else
            (return false ""))))
      (else
        (return false "")))
    (else
      (return false ""))))

(fn AIDescriptionbyID
  (params (ID :type Name))
  ;[1 1 1] Description for starting products (not from real players)
  (switch name ID
    (:Default
      (return "Default description."))
    (:Wood
      (return "Wood for a cheap price!"))
    (:stone
      (return "Boring stones..."))))

(fn GeneratePrdouctID
  (params (ItemString :type String))
  ;[1 1 1] Append item string with random integer to create Product ID
  (return (Utilities|String|Append ItemString "#" (Utilities|String|ToString(Integer) (Math|Random|RandomIntegerinRange 12 50000)))))

(fn GetInteractionWidgetRefI
  (return 0))