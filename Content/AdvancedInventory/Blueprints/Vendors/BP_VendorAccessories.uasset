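; BP_VendorAccessories is an accessories vendor actor in the inventory system that toggles a highlight render pass when focus changes.
; On BeginPlay it runs the parent logic and binds its Focus event to OnFocus.
; That event passes the focus state to SetRenderCustomDepth on the skeletal mesh and its static mesh parts.
; The construction script only calls the parent.
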(event Custom|Focus
  (params (Focus :type Boolean))
  (Rendering|SetRenderCustomDepth (Variables|Default|GetSkeletalMesh) Focus))

(event EventBeginPlay
  (|CallParentFunction)
  (EventDispatchers|BindEventtoOnFocus (delegate Custom|Focus)))

(fn ConstructionScript
  (|CallParentFunction))