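; Base-building component for the third-person character that previews and spawns buildables loaded from a data table.
; While build mode is on, a delayed loop traces from the camera on the buildable's channel and moves a collisionless ghost mesh.
; The ghost turns green on a hit, snapping to build boxes the hit actor reports, and red otherwise.
; Spawning places the actor at that transform and passes it the mesh, with one buildable ID also ending build mode.
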(event Custom|BuildDelay
  (bind _buildghost (Variables|Default|GetBUILDGHOST))
  (if (Variables|Default|GetIsBuildModeOn)
    (Utilities|FlowControl|Delay 0.01)
    (CallFunction|BuildCycle)
    (else
      (Variables|Default|SetIsBuildModeOn false)
      (Variables|Default|SetCanBuild false)
      (Utilities|IsValid _buildghost
        (:Is%20Valid
          (Default|DestroyCompnent (Variables|Default|GetPlayerReference) _buildghost))))))

(event Custom|LaunchBuild
  (if (Variables|Default|GetIsBuildModeOn)
    (CallFunction|StopBuildMode)
    (else
      (Variables|Default|SetIsBuildModeOn true)
      (CallFunction|BuildCycle))))

(event Custom|StopBuildMode
  (bind _buildghost (Variables|Default|GetBUILDGHOST))
  (Variables|Default|SetIsBuildModeOn false)
  (Variables|Default|SetCanBuild false)
  (Utilities|IsValid _buildghost
    (:Is%20Valid
      (Default|DestroyCompnent (Variables|Default|GetPlayerReference) _buildghost))))

(event EventBeginPlay
  (bind _asbp_third_person_character (Utilities|Casting|CastToBP_ThirdPersonCharacter (Components|GetOwner)))
  (Variables|Default|SetPlayerReference _asbp_third_person_character)
  (bind _outrownames (DataTable|GetDataTableRowNames "/Game/BASE_BUILDING/Building/BuildableDB.BuildableDB"))
  (for _array_element _outrownames
    (bind _returnvalue (Utilities|GetDataTableRow "/Game/BASE_BUILDING/Building/BuildableDB.BuildableDB" _array_element)
      (:then
        (Utilities|Array|Add (Variables|Default|GetBuildables) _returnvalue)))))

(fn SpawnBuildGhost
  (if (Variables|Default|Getoff%20build%20mode)
    (bind _returnvalue (Game|AddComponentbyClass (Variables|Default|GetPlayerReference) "/Script/Engine.StaticMeshComponent" false (Variables|Default|GetBuildTransform)))
    (bind _output_get (Variables|Default|SetBUILDGHOST _returnvalue))
    (Components|StaticMesh|SetStaticMesh _output_get (.mesh (Utilities|Array|Get(acopy) (Variables|Default|GetBuildables) (Variables|Default|GetBuildID))))
    (Collision|SetCollisionEnabled (Variables|Default|GetBUILDGHOST) "NoCollision")
    (if true
      (Development|PrintString "Hello"))))

(fn GiveBuildColor
  (params (IsGreen? :type Boolean))
  (bind _buildghost (Variables|Default|GetBUILDGHOST))
  (Variables|Default|SetCanBuild IsGreen?)
  (for _index (range (- (Rendering|Material|GetNumMaterials (Variables|Default|GetBUILDGHOST)) 1) 0)
    (if IsGreen?
      (Rendering|Material|SetMaterial _buildghost _index "/Game/BASE_BUILDING/TEXTURES/GreenColor.GreenColor")
      (else
        (Rendering|Material|SetMaterial _buildghost _index "/Game/BASE_BUILDING/TEXTURES/RedColor.RedColor"))))
  (Transformation|SetWorldTransform (Variables|Default|GetBUILDGHOST) (Variables|Default|GetBuildTransform) false false))

(fn BuildCycle
  (bind _camera (Variables|Default|GetCAMERA))
  (bind _buildghost (Variables|Default|GetBUILDGHOST))
  (bind _returnvalue (Transformation|GetWorldLocation _camera))
  (bind _returnvalue_2 (Math|Vector|GetForwardVector _camera))
  (bind (_outhit _returnvalue_3) (Collision|LineTraceByChannel (+ _returnvalue (* _returnvalue_2 350)) (+ _returnvalue (* _returnvalue_2 1000)) (.tracechannel (Utilities|Array|Get(acopy) (Variables|Default|GetBuildables) (Variables|Default|GetBuildID))) false 0 "None"))
  (if _returnvalue_3
    (Variables|Default|SetBuildTransform (Math|Transform|MakeTransform (.ImpactPoint (Collision|BreakHitResult _outhit)) (.rotation (Variables|Default|GetBuildTransform)) (.scale (Variables|Default|GetBuildTransform))))
    (Variables|Default|SetHit%20Actor (.HitActor (Collision|BreakHitResult _outhit)))
    (Variables|Default|SetHit%20Component (.HitComponent (Collision|BreakHitResult _outhit)))
    (Utilities|IsValid _buildghost
      (:Is%20Valid
        (bind (_found _transform) (CallFunction|DetectBuildBoxes))
        (if _found
          (Variables|Default|SetBuildTransform _transform))
        (CallFunction|GiveBuildColor true)
        (CallFunction|BuildDelay))
      (:Is%20Not%20Valid
        (CallFunction|SpawnBuildGhost :!label _label)
        (CallFunction|BuildDelay :!label _label_2)))
    (else
      (Variables|Default|SetBuildTransform (Math|Transform|MakeTransform (.TraceEnd (Collision|BreakHitResult _outhit)) (.rotation (Variables|Default|GetBuildTransform)) (.scale (Variables|Default|GetBuildTransform))))
      (Utilities|IsValid _buildghost
        (:Is%20Valid
          (CallFunction|GiveBuildColor false)
          (goto _label_2))
        (:Is%20Not%20Valid
          (goto _label))))))

(fn ChangeMesh
  (bind _buildghost (Variables|Default|GetBUILDGHOST))
  (Utilities|IsValid _buildghost
    (:Is%20Valid
      (Components|StaticMesh|SetStaticMesh _buildghost (.mesh (Utilities|Array|Get(acopy) (Variables|Default|GetBuildables) (Variables|Default|GetBuildID)))))))

(fn Spawnbuild
  (bind _returnvalue (Game|SpawnActorfromClass (.actor (Utilities|Array|Get(acopy) (Variables|Default|GetBuildables) (Variables|Default|GetBuildID))) (Variables|Default|GetBuildTransform) "Undefined" "MultiplyWithRoot" 0 0))
  (Class|BuildingInterface|SetMesh(Message) _returnvalue (.mesh (Utilities|Array|Get(acopy) (Variables|Default|GetBuildables) (Variables|Default|GetBuildID))))
  (if (== (Variables|Default|GetBuildID) 5)
    (Variables|Default|Setoff%20build%20mode false)
    (Variables|Default|SetIsBuildModeOn false)))

(fn DetectBuildBoxes
  (bind _boxes (Class|BuildingInterface|ReturnBoxes(Message) (Variables|Default|GetHit%20Actor)))
  (bind _array_element (Utilities|Array|ForEachLoopwithBreak _boxes :!label _label)
    (:LoopBody
      (if (== _array_element (Variables|Default|GetHit%20Component))
        (LocalVariables|SetLocalFound true)
        (goto _label Break)))
    (:Completed
      (return (LocalVariables|GetLocalFound) (Transformation|GetWorldTransform (Variables|Default|GetHit%20Component))))))